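; Base cultist enemy character that tracks its health, detects the player in melee range and deals strike damage.
; Each tick, a short forward debug-drawn line trace that hits a Player-tagged actor switches the AI controller's blackboard from chase to attack.
; Damage lowers the life pool and briefly flags a hit on the AnimBP; a hit at exactly zero life flags death, then destroys the actor.
; A box overlap applies damage to the player.
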(event OnComponentBeginOverlap(DamagePlayer_Box)
  (params (OverlappedComponent :type Primitive%20Component%20Object%20Reference) (OtherActor :type Actor%20Object%20Reference) (OtherComp :type Primitive%20Component%20Object%20Reference) (OtherBodyIndex :type Integer) (bFromSweep :type Boolean) (SweepResult :type Hit%20Result%20Structure%20%28by%20ref%29))
  ;[0.005983 0.07292 0.002262] Weapon damage to player
  (if (Actor|ActorHasTag OtherActor "Player")
    (Game|Damage|ApplyDamage (.PlayerChar_Ref (CallFunction|GetPlayerCharacterP)) (Variables|Life&Death|GetStrike_DMG) (Variables|Components|GetCultist%20Control%20Ref) self "/Script/Engine.DamageType")))

(event Custom|OnTakeAnyDamage_Enter
  (params (DamagedActor :type Actor%20Object%20Reference) (Damage :type Float%20%28single-precision%29) (DamageType :type Damage%20Type%20Object%20Reference) (InstigatedBy :type Controller%20Object%20Reference) (DamageCauser :type Actor%20Object%20Reference))
  ;[0.007087 0.01363 0.224] BEGIN PLAY
  ;;[0 0 0] Upon Ghouly taking damage
  (if (and (not (Variables|Life&Death|GetbIsDead?)) (!= (Variables|Life&Death|GetLifePool) 0.0))
    (Variables|Life&Death|SetLifePool (- (Variables|Life&Death|GetLifePool) Damage))
    (bind _output_get (Variables|Life&Death|SetbBeenHit? true))
    (Variables|/Game/Character/BSP_ZombieAnims/Animations/ABP_Cultist.ABP_Cultist_C|SetbBeenHit? (Variables|Components|GetCultist%20Anim%20BP%20Ref) _output_get)
    (Utilities|FlowControl|Delay 1.0)
    (Variables|Life&Death|SetbBeenHit? false)
    (else
      (bind _output_get_2 (Variables|Life&Death|SetbIsDead? true))
      (Variables|/Game/Character/BSP_ZombieAnims/Animations/ABP_Cultist.ABP_Cultist_C|SetbHasDied? (Variables|Components|GetCultist%20Anim%20BP%20Ref) _output_get_2)
      (Utilities|FlowControl|Delay 2.0)
      (Actor|DestroyActor DamagedActor))))

(event EventBeginPlay
  (bind _self self)
  (bind (_cultistchar_ref _cultistcontrol_ref _cultistanimbp_ref) (CallFunction|GetCultistRef _self))
  ;[0.007087 0.01363 0.224] BEGIN PLAY
  (Variables|Life&Death|SetLifePool (Variables|Life&Death|GetMax_LifePool))
  (Variables|Components|SetCultist%20Control%20Ref _cultistcontrol_ref)
  (Variables|Components|SetCultist%20Anim%20BP%20Ref _cultistanimbp_ref)
  (EventDispatchers|AssignOnTakeAnyDamage _self (delegate Custom|OnTakeAnyDamage_Enter)))

(event EventTick
  (params (DeltaSeconds :type Float%20%28single-precision%29))
  ;[0.1198 0.09488 0] PER FRAME EVENTS
  (CallFunction|FAimatEnemy))

(fn ConstructionScript)

(fn FAimatEnemy
  (bind _self self)
  (bind _self_2 self)
  (bind _cultist_control_ref (Variables|Components|GetCultist%20Control%20Ref))
  (bind _returnvalue (Transformation|GetActorLocation _self_2))
  ;[0.03737 0 0.1302] Seeking attack
  (bind _outhit (Collision|LineTraceByChannel _returnvalue (+ _returnvalue (* (Math|Vector|GetForwardVector (Transformation|GetActorRotation _self_2)) 1.5e+02)) "TraceTypeQuery4" false (Utilities|Array|MakeArray _self (.CultistChar_Ref (CallFunction|GetCultistRef _self))) "ForDuration"))
  (if (.bBlockingHit (Collision|BreakHitResult _outhit))
    (if (Actor|ActorHasTag (.HitActor (Collision|BreakHitResult _outhit)) "Player")
      (AI|Components|Blackboard|SetValueasBool (AI|GetBlackboard _cultist_control_ref) (Utilities|Name|MakeLiteralName "bAttack?") (.bBlockingHit (Collision|BreakHitResult _outhit)))
      (AI|Components|Blackboard|SetValueasBool (AI|GetBlackboard (Variables|Components|GetCultist%20Control%20Ref)) (Utilities|Name|MakeLiteralName "bTakeChase?") (not (.bBlockingHit (Collision|BreakHitResult _outhit))))
      (elif (not (.bBlockingHit (Collision|BreakHitResult _outhit)))
        (Default|ExitAttack _cultist_control_ref self)))))