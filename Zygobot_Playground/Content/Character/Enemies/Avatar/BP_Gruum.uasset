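; BP_Gruum is an enemy character Blueprint that handles damage and death for Gruum.
; BeginPlay fills GruumLifeSpan from its maximum and binds a handler to any damage received.
; Each hit subtracts life and raises BeenHit for a second.
; A hit arriving when life is exactly zero sets IsDead and destroys the actor after a short delay; negative life does not trigger death.
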(event Custom|OnTakeAnyDamage_Event_0
  (params (DamagedActor :type Actor%20Object%20Reference) (Damage :type Float%20%28single-precision%29) (DamageType :type Damage%20Type%20Object%20Reference) (InstigatedBy :type Controller%20Object%20Reference) (DamageCauser :type Actor%20Object%20Reference))
  ;[0.1667 0 0] Take damage event
  (if (and (not (Variables|LifeSpan|GetbIsDead?)) (!= (Variables|LifeSpan|GetGruum_LifeSpan) 0.0))
    (Variables|LifeSpan|SetGruum_LifeSpan (- (Variables|LifeSpan|GetGruum_LifeSpan) Damage))
    (Variables|LifeSpan|SetbBeenHit? true)
    (Utilities|FlowControl|Delay 1.0)
    (Variables|LifeSpan|SetbBeenHit? false)
    (else
      (Variables|LifeSpan|SetbIsDead? true)
      (Utilities|FlowControl|Delay 1.5)
      (Actor|DestroyActor DamagedActor))))

(event EventBeginPlay
  ;[0 0.0182 0.1562] BEGIN PLAY
  (Variables|LifeSpan|SetGruum_LifeSpan (Variables|LifeSpan|GetGruum_MaxLifeSPan))
  (EventDispatchers|AssignOnTakeAnyDamage (delegate Custom|OnTakeAnyDamage_Event_0)))

(event Collision|EventActorBeginOverlap
  (params (OtherActor :type Actor%20Object%20Reference)))

(event EventTick
  (params (DeltaSeconds :type Float%20%28single-precision%29)))

(fn ConstructionScript)