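; BP_ClotWorm is an enemy worm that takes damage, shows a hurt reaction and dies.
; At BeginPlay it fills its life pool, binds to any damage and caches its control and AnimBP references.
; Damage lowers life and briefly pulses the AnimBP's Hurt flag; a hit at exactly zero life sets HasDied, then destroys the actor after a delay.
; Pistol bullet overlaps on the Box only update those animation flags.
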(event OnComponentBeginOverlap(Box)
  (params (OverlappedComponent :type Primitive%20Component%20Object%20Reference) (OtherActor :type Actor%20Object%20Reference) (OtherComp :type Primitive%20Component%20Object%20Reference) (OtherBodyIndex :type Integer) (bFromSweep :type Boolean) (SweepResult :type Hit%20Result%20Structure%20%28by%20ref%29))
  (bind _clot_worm_anim_bp_ref (Variables|Components|GetClot%20Worm%20Anim%20BP%20Ref))
  ;[0.1562 0 0] Worm gets hit with bullet
  (if (Actor|ActorHasTag OtherActor "Pistol_Bullet")
    (if (!= (Variables|LifeSpan|GetWorm_LifeSpan) 0.0)
      (Variables|/Game/Character/InfinityBladeAdversaries/Enemy/Enemy_Clot_Worm/Enemy_Clot_Worm_Animation/ABP_ClotWorm.ABP_ClotWorm_C|SetbHurt? _clot_worm_anim_bp_ref (Variables|LifeSpan|GetbBeenHit?))
      (else
        (bind _output_get (Variables|LifeSpan|SetbIsDead? true))
        (Variables|/Game/Character/InfinityBladeAdversaries/Enemy/Enemy_Clot_Worm/Enemy_Clot_Worm_Animation/ABP_ClotWorm.ABP_ClotWorm_C|SetbHasDied? _clot_worm_anim_bp_ref _output_get)))))

(event Custom|OnTakeAnyDamage_Event_0
  (params (DamagedActor :type Actor%20Object%20Reference) (Damage :type Float%20%28single-precision%29) (DamageType :type Damage%20Type%20Object%20Reference) (InstigatedBy :type Controller%20Object%20Reference) (DamageCauser :type Actor%20Object%20Reference))
  ;[0.1667 0 0] Take damage event
  (if (and (not (Variables|LifeSpan|GetbIsDead?)) (!= (Variables|LifeSpan|GetWorm_LifeSpan) 0.0))
    (Variables|LifeSpan|SetWorm_LifeSpan (- (Variables|LifeSpan|GetWorm_LifeSpan) Damage))
    (bind _output_get (Variables|LifeSpan|SetbBeenHit? true))
    (Variables|/Game/Character/InfinityBladeAdversaries/Enemy/Enemy_Clot_Worm/Enemy_Clot_Worm_Animation/ABP_ClotWorm.ABP_ClotWorm_C|SetbHurt? (Variables|Components|GetClot%20Worm%20Anim%20BP%20Ref) _output_get)
    (Utilities|FlowControl|Delay 1.0)
    (bind _output_get_2 (Variables|LifeSpan|SetbBeenHit? false))
    (Variables|/Game/Character/InfinityBladeAdversaries/Enemy/Enemy_Clot_Worm/Enemy_Clot_Worm_Animation/ABP_ClotWorm.ABP_ClotWorm_C|SetbHurt? (Variables|Components|GetClot%20Worm%20Anim%20BP%20Ref) _output_get_2)
    (else
      (if (not (Variables|LifeSpan|GetbIsDead?))
        _
        (else
          _))
      (bind _output_get_3 (Variables|LifeSpan|SetbIsDead? true))
      (Variables|/Game/Character/InfinityBladeAdversaries/Enemy/Enemy_Clot_Worm/Enemy_Clot_Worm_Animation/ABP_ClotWorm.ABP_ClotWorm_C|SetbHasDied? (Variables|Components|GetClot%20Worm%20Anim%20BP%20Ref) _output_get_3)
      (Utilities|FlowControl|Delay 1.5)
      (Actor|DestroyActor DamagedActor))))

(event EventBeginPlay
  (bind _self self)
  (bind (_clotwormchar_ref _clotwormcontrol_ref _clotwormanimbp_ref) (CallFunction|GetClotWormRef _self))
  ;[0 0.0182 0.1562] BEGIN PLAY
  (Variables|LifeSpan|SetWorm_LifeSpan (Variables|LifeSpan|GetWorm_MaxLifeSPan))
  (EventDispatchers|AssignOnTakeAnyDamage (delegate Custom|OnTakeAnyDamage_Event_0))
  (Variables|Components|SetClot%20Worm%20Control%20Ref _clotwormcontrol_ref)
  (Variables|Components|SetClot%20Worm%20Anim%20BP%20Ref _clotwormanimbp_ref))

(event Collision|EventActorBeginOverlap
  (params (OtherActor :type Actor%20Object%20Reference)))

(event EventTick
  (params (DeltaSeconds :type Float%20%28single-precision%29)))

(fn ConstructionScript)