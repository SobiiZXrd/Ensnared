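; AI controller for the Ghouly Ghast enemy, running its behavior tree and starting it in patrol.
; Perception updates pass through hearing, sight and damage handlers, which write chase location, enemy and state flags to the Blackboard.
; Sight and damage require the Player tag; hearing checks stimulus age instead and flags investigation.
; Enter and Exit Attack events update the anim Blueprint's attack flag, with exit also clearing the Blackboard key.
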(event OnTargetPerceptionUpdated(AIPerception)
  (params (Actor :type Actor%20Object%20Reference) (Stimulus :type AI%20Stimulus%20Structure))
  ;[0 0 0] AI Perception update variable manipulation
  (Variables|PerceptionSystem|SetPerceivedActor Actor)
  (bind _output_get (Variables|PerceptionSystem|SetStimulus Stimulus))
  (PerceptionSystem|FHandleSoundSense _output_get)
  (PerceptionSystem|FHandleSightSense (Variables|PerceptionSystem|GetStimulus))
  (PerceptionSystem|FHandleDamageSense (Variables|PerceptionSystem|GetStimulus))
  (if (>= (.Age (Utilities|Struct|BreakAIStimulus (Variables|PerceptionSystem|GetStimulus))) 3.0)
    _))

(event Custom|Exit_Attack
  (params (ControlledPawn_Ref :type Pawn%20Object%20Reference))
  ;[0.0186 0.06771 0.01242] Enter and exit attack mode
  (AI|Components|Blackboard|SetValueasBool (Variables|Default|GetGhouly_BlackboardRef) (Utilities|Name|MakeLiteralName "bAttack?") false)
  (Variables|/Game/Character/InfinityBladeAdversaries/Enemy/Enemy_Master_Grunt/Enemy_Master_Grunt_Animation/ABP_GM.ABP_GM_C|SetbIsAttacking? (.GhoulyAnimBP_Ref (CallFunction|GetGhoulGhastRef ControlledPawn_Ref)) false))

(event Custom|Enter_Attack
  (params (ControlledPawn_Ref :type Pawn%20Object%20Reference))
  ;[0.0186 0.06771 0.01242] Enter and exit attack mode
  (Variables|/Game/Character/InfinityBladeAdversaries/Enemy/Enemy_Master_Grunt/Enemy_Master_Grunt_Animation/ABP_GM.ABP_GM_C|SetbIsAttacking? (.GhoulyAnimBP_Ref (CallFunction|GetGhoulGhastRef ControlledPawn_Ref)) (ScalableFloat|GetValueasBool (Variables|Default|GetGhouly_BlackboardRef) (Utilities|Name|MakeLiteralName "bAttack?"))))

(event EventBeginPlay
  ;[0 0.001457 0.1146] BEGIN PLAY
  (AI|RunBehaviorTree self "/Game/Character/Enemies/BT/BT_GhoulyGhast.BT_GhoulyGhast")
  (bind _output_get (Variables|Default|SetGhouly_BlackboardRef (AI|GetBlackboard self)))
  (Class|BlackboardComponent|SetValueasInt _output_get (Utilities|Name|MakeLiteralName "PatrolIndex"))
  (AI|Components|Blackboard|SetValueasBool (Variables|Default|GetGhouly_BlackboardRef) (Utilities|Name|MakeLiteralName "bPatrol?") true))

(event EventTick
  (params (DeltaSeconds :type Float%20%28single-precision%29))
  ;[0.1147 0.1354 0.00598] PER FRAME EVENTS
)

(fn ConstructionScript)

(fn FSetEnemy
  (params (PerceivedActor :type Actor%20Object%20Reference))
  (bind _ghouly_blackboardref (Variables|Default|GetGhouly_BlackboardRef))
  (if (!= PerceivedActor 0)
    (AI|Components|Blackboard|SetValueasObject _ghouly_blackboardref (Utilities|Name|MakeLiteralName "Enemy") PerceivedActor)
    (AI|Components|Blackboard|SetValueasBool _ghouly_blackboardref (Utilities|Name|MakeLiteralName "bTakeChase?") true)
    (AI|Components|Blackboard|SetValueasBool _ghouly_blackboardref (Utilities|Name|MakeLiteralName "bPatrol?") false)))

(fn FHandleSightSense
  (params (Stimulus :type AI%20Stimulus%20Structure%20%28by%20ref%29))
  (bind _ghouly_blackboardref (Variables|Default|GetGhouly_BlackboardRef))
  (bind (_age _expirationage _strength _stimuluslocation _receiverlocation _tag _bsuccessfullysensed) (Utilities|Struct|BreakAIStimulus (Variables|PerceptionSystem|GetStimulus)))
  ;[0.03678 0.01107 0.0625] Does Ghouly see its enemy?
  (bind _returnvalue (Class|AIPerceptionSystem|GetSenseClassforStimulus Stimulus))
  (Variables|PerceptionSystem|GetPerceivedActor
    (:then
      (if (== _returnvalue "/Script/AIModule.AISense_Sight")
        (if (and (Actor|ActorHasTag (Variables|PerceptionSystem|GetPerceivedActor) "Player") _bsuccessfullysensed)
          (AI|Components|Blackboard|SetValueasVector _ghouly_blackboardref (Utilities|Name|MakeLiteralName "Chase_Vector") _stimuluslocation)
          (else
            (bind _output_get (Variables|PerceptionSystem|SetPerceivedActor 0))
            (AI|Components|Blackboard|SetValueasObject _ghouly_blackboardref (Utilities|Name|MakeLiteralName "Enemy") _output_get)))
        (AI|Components|Blackboard|SetValueasBool _ghouly_blackboardref (Utilities|Name|MakeLiteralName "bTakeChase?") _bsuccessfullysensed)
        (PerceptionSystem|FSetEnemy (Variables|PerceptionSystem|GetPerceivedActor))))
    (:else
      (Variables|PerceptionSystem|SetPerceivedActor 0))))

(fn FHandleSoundSense
  (params (Stimulus :type AI%20Stimulus%20Structure%20%28by%20ref%29))
  (bind _ghouly_blackboardref (Variables|Default|GetGhouly_BlackboardRef))
  (bind (_age _expirationage _strength _stimuluslocation _receiverlocation _tag _bsuccessfullysensed) (Utilities|Struct|BreakAIStimulus (Variables|PerceptionSystem|GetStimulus)))
  ;[0.0638 0.01823 0.1094] Does Ghouly hear its enemy?
  (bind _returnvalue (Class|AIPerceptionSystem|GetSenseClassforStimulus Stimulus))
  (Variables|PerceptionSystem|GetPerceivedActor
    (:then
      (if (== _returnvalue "/Script/AIModule.AISense_Hearing")
        (if (and _bsuccessfullysensed (< _age 3.0))
          (AI|Components|Blackboard|SetValueasVector _ghouly_blackboardref (Utilities|Name|MakeLiteralName "Chase_Vector") _stimuluslocation)
          (PerceptionSystem|FSetEnemy (Variables|PerceptionSystem|GetPerceivedActor))
          (AI|Components|Blackboard|SetValueasBool _ghouly_blackboardref (Utilities|Name|MakeLiteralName "bInvestigate?") _bsuccessfullysensed :!label _label)
          (elif (>= _age 3.0)
            (bind _output_get (Variables|PerceptionSystem|SetPerceivedActor 0))
            (AI|Components|Blackboard|SetValueasObject _ghouly_blackboardref (Utilities|Name|MakeLiteralName "Enemy") _output_get)
            (goto _label)))
        (else
          (Variables|PerceptionSystem|SetPerceivedActor 0))))
    (:else
      (Variables|PerceptionSystem|SetPerceivedActor 0))))

(fn FHandleDamageSense
  (params (Stimulus :type AI%20Stimulus%20Structure%20%28by%20ref%29))
  (bind (_age _expirationage _strength _stimuluslocation _receiverlocation _tag _bsuccessfullysensed) (Utilities|Struct|BreakAIStimulus (Variables|PerceptionSystem|GetStimulus)))
  (bind _returnvalue (Class|AIPerceptionSystem|GetSenseClassforStimulus Stimulus))
  (Variables|PerceptionSystem|GetPerceivedActor
    (:then
      (if (== _returnvalue "/Script/AIModule.AISense_Damage")
        (if (and (Actor|ActorHasTag (Variables|PerceptionSystem|GetPerceivedActor) "Player") _bsuccessfullysensed)
          (AI|Components|Blackboard|SetValueasVector (Variables|Default|GetGhouly_BlackboardRef) (Utilities|Name|MakeLiteralName "Chase_Vector") _stimuluslocation)
          (else
            (Variables|PerceptionSystem|SetPerceivedActor 0)))
        (PerceptionSystem|FSetEnemy (Variables|PerceptionSystem|GetPerceivedActor))))
    (:else
      (Variables|PerceptionSystem|SetPerceivedActor 0))))