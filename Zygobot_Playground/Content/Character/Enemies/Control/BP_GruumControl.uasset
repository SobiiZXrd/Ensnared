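; AI controller for the Gruum enemy that runs its behavior tree and starts it patrolling through blackboard keys.
; Perception updates go to hearing or sight handlers; recent sounds set the chase location, enemy, and chase and investigate flags.
; The sight handler re-checks for the hearing sense, so sight stimuli never trigger its chase logic.
; Enter and exit attack events sync the attack state to Gruum's animation Blueprint.
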(event OnTargetPerceptionUpdated(AIPerception)
  (params (Actor :type Actor%20Object%20Reference) (Stimulus :type AI%20Stimulus%20Structure))
  ;[0 0 0] AI Perception update variable manipulation
  (Variables|PerceptionSystem|SetPerceivedActor Actor)
  (bind _output_get (Variables|PerceptionSystem|SetStimulus Stimulus))
  (bind _returnvalue (Class|AIPerceptionSystem|GetSenseClassforStimulus _output_get))
  (if (== _returnvalue "/Script/AIModule.AISense_Hearing")
    (CallFunction|FHadleSoundSense (Variables|PerceptionSystem|GetStimulus))
    (elif (== _returnvalue "/Script/AIModule.AISense_Sight")
      (CallFunction|FHandleSightSense (Variables|PerceptionSystem|GetStimulus)))))

(event Custom|Enter_Attack
  (params (Controlled%20Pawn :type Pawn%20Object%20Reference))
  ;[0.1354 0 0] Enter and Exit Attack sequence
  (Variables|/Game/UndeadPack/Lich/Animations/AnimBP_Gruum.AnimBP_Gruum_C|SetbIsAttacking? (.Gruum_AnimBPRef (CallFunction|GetGruumRef Controlled%20Pawn)) (ScalableFloat|GetValueasBool (Variables|Default|GetGruum_BlackboardRef) (Utilities|Name|MakeLiteralName "bAttack?"))))

(event Custom|Exit_Attack
  (params (Controlled%20Pawn :type Pawn%20Object%20Reference))
  ;[0.1354 0 0] Enter and Exit Attack sequence
  (AI|Components|Blackboard|SetValueasBool (Variables|Default|GetGruum_BlackboardRef) (Utilities|Name|MakeLiteralName "bAttack?") false)
  (Variables|/Game/UndeadPack/Lich/Animations/AnimBP_Gruum.AnimBP_Gruum_C|SetbIsAttacking? (.Gruum_AnimBPRef (CallFunction|GetGruumRef Controlled%20Pawn)) false))

(event EventBeginPlay
  (bind _self self)
  ;[0.01447 0.008387 0.1875] BEGIN PLAY
  (AI|RunBehaviorTree _self "/Game/Character/Enemies/BT/BT_Gruum.BT_Gruum")
  (Variables|Default|SetGruum_BlackboardRef (AI|GetBlackboard _self))
  (Class|BlackboardComponent|SetValueasInt (Variables|Default|GetGruum_BlackboardRef) (Utilities|Name|MakeLiteralName "PatrolIndex"))
  (AI|Components|Blackboard|SetValueasBool (Variables|Default|GetGruum_BlackboardRef) (Utilities|Name|MakeLiteralName "bPatrol?") true))

(event EventTick
  (params (DeltaSeconds :type Float%20%28single-precision%29)))

(fn ConstructionScript)

(fn FHadleSoundSense
  (params (Stimulus :type AI%20Stimulus%20Structure))
  (bind _gruum_blackboardref (Variables|Default|GetGruum_BlackboardRef))
  (bind (_age _expirationage _strength _stimuluslocation _receiverlocation _tag _bsuccessfullysensed) (Utilities|Struct|BreakAIStimulus (Variables|PerceptionSystem|GetStimulus)))
  ;[0.04469 0.01211 0.07292] Does Gruum hear the player?
  (bind _returnvalue (Class|AIPerceptionSystem|GetSenseClassforStimulus Stimulus))
  (Variables|PerceptionSystem|GetPerceivedActor
    (:then
      (if (== _returnvalue "/Script/AIModule.AISense_Hearing")
        (if (and _bsuccessfullysensed (< _age 3.0))
          (AI|Components|Blackboard|SetValueasVector _gruum_blackboardref (Utilities|Name|MakeLiteralName "Chase_Vector") _stimuluslocation)
          (CallFunction|FSetEnemy (Variables|PerceptionSystem|GetPerceivedActor))
          (AI|Components|Blackboard|SetValueasBool _gruum_blackboardref (Utilities|Name|MakeLiteralName "bInvestigate?") _bsuccessfullysensed :!label _label)
          (elif (>= _age 3.0)
            (bind _output_get (Variables|PerceptionSystem|SetPerceivedActor 0))
            (AI|Components|Blackboard|SetValueasObject _gruum_blackboardref (Utilities|Name|MakeLiteralName "Enemy") _output_get)
            (goto _label)))
        (else
          (Variables|PerceptionSystem|SetPerceivedActor 0))))
    (:else
      (Variables|PerceptionSystem|SetPerceivedActor 0))))

(fn FSetEnemy
  (params (Enemy :type Actor%20Object%20Reference))
  (bind _gruum_blackboardref (Variables|Default|GetGruum_BlackboardRef))
  ;[0.05717 0.02245 0.09375] Setting Enemy
  (if (!= Enemy 0)
    (AI|Components|Blackboard|SetValueasObject _gruum_blackboardref (Utilities|Name|MakeLiteralName "Enemy") Enemy)
    (AI|Components|Blackboard|SetValueasBool _gruum_blackboardref (Utilities|Name|MakeLiteralName "bTakeChase?") true)
    (AI|Components|Blackboard|SetValueasBool _gruum_blackboardref (Utilities|Name|MakeLiteralName "bPatrol?") false)))

(fn FHandleSightSense
  (params (Stimulus :type AI%20Stimulus%20Structure))
  (bind _gruum_blackboardref (Variables|Default|GetGruum_BlackboardRef))
  (bind _bsuccessfullysensed (Utilities|Struct|BreakAIStimulus (Variables|PerceptionSystem|GetStimulus)))
  ;[0.03705 0.002376 0.08333] Function called when player or actions the player took have been heard by this AI
  (bind _returnvalue (Class|AIPerceptionSystem|GetSenseClassforStimulus Stimulus))
  (if (== _returnvalue "/Script/AIModule.AISense_Hearing")
    (Variables|PerceptionSystem|GetPerceivedActor
      (:then
        (if (and (Actor|ActorHasTag (Variables|PerceptionSystem|GetPerceivedActor) "Player") _bsuccessfullysensed)
          (AI|Components|Blackboard|SetValueasVector _gruum_blackboardref (Utilities|Name|MakeLiteralName "Chase_Vector") "0, 0, 0")
          (CallFunction|FSetEnemy (Variables|PerceptionSystem|GetPerceivedActor))
          (else
            (bind _output_get (Variables|PerceptionSystem|SetPerceivedActor 0))
            (AI|Components|Blackboard|SetValueasObject _gruum_blackboardref (Utilities|Name|MakeLiteralName "Enemy") _output_get)))
        (AI|Components|Blackboard|SetValueasBool _gruum_blackboardref (Utilities|Name|MakeLiteralName "bTakeChase?") _bsuccessfullysensed))
      (:else
        (Variables|PerceptionSystem|SetPerceivedActor 0)))))