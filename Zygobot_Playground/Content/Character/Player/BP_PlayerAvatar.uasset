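; First-person player avatar for an escape game with clue collecting and a shape puzzle, handling HUD, damage, flashlight and interaction.
; BeginPlay creates the HUD widget, which shows health, an interact prompt and a clue count that briefly flashes green on update.
; A per-tick camera line trace finds "Interactable"-tagged targets for the Interact input to message.
; That trace also sets the Cone, Sphere and Cube possession flags from component tags.
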(event Custom|Event_UpdateHUD
  (params (CluesFound :type Integer))
  (bind _w_updateclue_ref (Variables|HUDUI|GetW_UpdateClue_Ref))
  (bind _cluesfound_cluecount (Variables|/Game/Systems/UI_HUD/W_PlayerHUD_UI.W_PlayerHUD_UI_C|GetCluesFound_ClueCount _w_updateclue_ref))
  ;[1 0 0] Event to update clues for escape
  (Variables|/Game/Systems/UI_HUD/W_PlayerHUD_UI.W_PlayerHUD_UI_C|SetCluesFound_Text _w_updateclue_ref (Utilities|Text|ToText(Integer) CluesFound))
  (Class|EditableTextBox|SetForegroundColor _cluesfound_cluecount "(R=0.000000,G=0.750000,B=0.063900,A=1.000000)")
  (Utilities|FlowControl|Delay 0.7)
  (Class|EditableTextBox|SetForegroundColor _cluesfound_cluecount "(R=1.000000,G=1.000000,B=1.000000,A=1.000000)"))

(event Custom|OnTakeAnyDamage_Enter
  (params (DamagedActor :type Actor%20Object%20Reference) (Damage :type Float%20%28single-precision%29) (DamageType :type Damage%20Type%20Object%20Reference) (InstigatedBy :type Controller%20Object%20Reference) (DamageCauser :type Actor%20Object%20Reference))
  ;[0.04638 0.2073 1] BEGIN PLAY
  ;;[0 0 0] Player taking damage bind event on begin play
  (Utilities|FlowControl|DoOnce false
    (:Completed
      (if (!= (Variables|PlayerHealthVariables|GetPlayer_CurHealth) 0.0)
        (bind _output_get (Variables|PlayerHealthVariables|SetPlayer_CurHealth (- (Variables|PlayerHealthVariables|GetPlayer_CurHealth) Damage)))
        (HUD_UI|UpdateHealth _output_get)
        (CallFunction|ResetDamageTaken)))))

(event Custom|Reset_DamageTaken
  ;[0.04638 0.2073 1] BEGIN PLAY
  ;;[0 0 0] Player taking damage bind event on begin play
)

(event EventBeginPlay
  ;[0.04638 0.2073 1] BEGIN PLAY
  ;;[0.01562 0.01562 0.01562] Adding Player HUD/UI to viewport
  (bind _returnvalue (UserInterface|CreateWidget "/Game/Systems/UI_HUD/W_PlayerHUD_UI.W_PlayerHUD_UI_C"))
  (bind _output_get (Variables|HUDUI|SetW_UpdateClue_Ref _returnvalue))
  (Widget|SetVisibility (Variables|/Game/Systems/UI_HUD/W_PlayerHUD_UI.W_PlayerHUD_UI_C|GetInteract_Text _output_get) (Variables|InteractSystem|GetInteractText_SetHidden))
  (UserInterface|Viewport|AddtoViewport _output_get 0)
  (HUD_UI|UpdateHealth (Variables|PlayerHealthVariables|GetPlayer_CurHealth))
  ;;[0 0 0] Door Puzzle piece control
  (Variables|DoorPuzzleInteraction|SetbHasCone false)
  (Variables|DoorPuzzleInteraction|SetbHasSphere false)
  (Variables|DoorPuzzleInteraction|SetbHasCube false)
  (EventDispatchers|AssignOnTakeAnyDamage (delegate Custom|OnTakeAnyDamage_Enter)))

(event EventTick
  (params (DeltaSeconds :type Float%20%28single-precision%29))
  ;[1 0 0] PER FRAME EVENTS
  ;;[0 0 0] Object interaction line trace
  (InteractionSystemFunctions|SeekingInteractable))

(event Input|ActionEvents|InputActionInteract
  (params (Key :type Key%20Structure :default "None"))
  ;[0.01531 0.151 0.02574] Press "E" To Interact
  (:Pressed
    (Utilities|FlowControl|Sequence
      (:then_0
        (bind _interactable (Variables|InteractSystem|GetInteractable)
          (:then
            (Class|IInteract|Interact(Message) _interactable))
          (:else
            (Variables|InteractSystem|SetInteractable 0)))))))

(event Input|ActionEvents|InputActionFlashlight
  (params (Key :type Key%20Structure :default "None"))
  (bind _spotlight (Variables|Default|GetSpotLight))
  ;[0.125 0.09834 0] Turn flashlight on or of be pressing "F"
  (:Pressed
    (Utilities|FlowControl|FlipFlop
      (:A
        (Rendering|SetVisibility _spotlight false false))
      (:B
        (Rendering|SetVisibility _spotlight true false)))))

(fn ConstructionScript)

(fn SetInteractObject
  (params (Interactable :type Actor%20Object%20Reference))
  ;[0.6083 0.1768 1] Once the line trace deems an object as interactable (Actor Has Tag: Interactable) this function will set the Interactable object reference tothe "HitActor"
  (if (!= Interactable 0)
    (bind _output_get (Variables|InteractSystem|SetInteractable Interactable))
    (return _output_get)
    (else
      (Widget|SetVisibility (Variables|/Game/Systems/UI_HUD/W_PlayerHUD_UI.W_PlayerHUD_UI_C|GetInteract_Text (Variables|HUDUI|GetW_UpdateClue_Ref)) (Variables|InteractSystem|GetInteractText_SetHidden)))))

(fn SeekingInteractable
  (bind _firstpersoncamera (Variables|Default|GetFirstPersonCamera))
  (bind _returnvalue (Transformation|GetWorldLocation _firstpersoncamera))
  ;[0.6037 0.1874 1] Line tracing seeking interactables in the player's environment
  (bind _outhit (Collision|LineTraceByChannel _returnvalue (+ (* (Math|Vector|GetForwardVector (Transformation|GetWorldRotation _firstpersoncamera)) 2e+02) _returnvalue) "TraceTypeQuery3" false (Utilities|Array|MakeArray self) "None" true "(R=0.030084,G=1.000000,B=0.000000,A=1.000000)" "(R=1.000000,G=0.000000,B=0.009744,A=1.000000)"))
  (Utilities|IsValid (.HitActor (Collision|BreakHitResult _outhit))
    (:Is%20Valid
      (if (and (.bBlockingHit (Collision|BreakHitResult _outhit)) (or (Actor|ActorHasTag (.HitActor (Collision|BreakHitResult _outhit)) "Interactable") (Components|ComponentHasTag (.HitComponent (Collision|BreakHitResult _outhit)) "Interactable")))
        (Widget|SetVisibility (Variables|/Game/Systems/UI_HUD/W_PlayerHUD_UI.W_PlayerHUD_UI_C|GetInteract_Text (Variables|HUDUI|GetW_UpdateClue_Ref)) "Visible")
        (InteractionSystemFunctions|SetInteractObject (.HitActor (Collision|BreakHitResult _outhit)))
        (Utilities|IsValid (.HitComponent (Collision|BreakHitResult _outhit))
          (:Is%20Valid
            (InteractionSystemFunctions|SetInteractObject (Components|GetOwner (.HitComponent (Collision|BreakHitResult _outhit))))
            (if (Components|ComponentHasTag (.HitComponent (Collision|BreakHitResult _outhit)) "Cone")
              (Variables|DoorPuzzleInteraction|SetbHasCone true)
              (elif (Components|ComponentHasTag (.HitComponent (Collision|BreakHitResult _outhit)) "Sphere")
                (Variables|DoorPuzzleInteraction|SetbHasSphere true)
                (elif (Components|ComponentHasTag (.HitComponent (Collision|BreakHitResult _outhit)) "Cube")
                  (Variables|DoorPuzzleInteraction|SetbHasCube true)))))
          (:Is%20Not%20Valid
            (Variables|InteractSystem|SetInteractable 0)
            (Widget|SetVisibility (Variables|/Game/Systems/UI_HUD/W_PlayerHUD_UI.W_PlayerHUD_UI_C|GetInteract_Text (Variables|HUDUI|GetW_UpdateClue_Ref)) (Variables|InteractSystem|GetInteractText_SetHidden))))
        (else
          (Variables|InteractSystem|SetInteractable 0 :!label _label)
          (Widget|SetVisibility (Variables|/Game/Systems/UI_HUD/W_PlayerHUD_UI.W_PlayerHUD_UI_C|GetInteract_Text (Variables|HUDUI|GetW_UpdateClue_Ref)) (Variables|InteractSystem|GetInteractText_SetHidden)))))
    (:Is%20Not%20Valid
      (goto _label))))

(fn UpdateHealth
  (params (Current_PlayerHealth :type Float%20%28double-precision%29))
  (Progress|SetPercent (Variables|/Game/Systems/UI_HUD/W_PlayerHUD_UI.W_PlayerHUD_UI_C|GetHUD_PlayerHealth (Variables|HUDUI|GetW_UpdateClue_Ref)) (/ Current_PlayerHealth 1e+02)))

(fn FNotifySound
  (params (Footstep :type Anim%20Notify%20Object%20Reference))
  ;[0.08734 0 0.1927] When the player steps can be heard by enemies
  (Class|AudioLinkBlueprintInterface|SetLinkSound(Message) (Variables|Default|GetAIPerceptionStimuliSource) "/Game/Character/FPS_AnimBP_v2/Audio/Footsteps/Concrete/WAV/WAV_Footstep_Concrete_Walk01.WAV_Footstep_Concrete_Walk01"))