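; Player character Blueprint for what appears to be an escape game with clues, a shape-based door puzzle and enemies that hear footsteps.
; A per-tick camera line trace finds "Interactable" tagged targets, shows the HUD prompt, stores the Interact target and flags Cone, Sphere or Cube on sight.
; Damage updates the health bar and blood overlay, with death animation then actor destruction at zero health.
; It also handles flashlight toggling and clue counter updates.
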(event Custom|Event_UpdateHUD
  (params (CluesFound :type Integer))
  (bind _w_updateclue_ref (Variables|Default|GetW_UpdateClue_Ref))
  (bind _cluesfound_cluecount (Variables|/Game/Systems/UI_HUD/W_PlayerHUD_UI.W_PlayerHUD_UI_C|GetCluesFound_ClueCount _w_updateclue_ref))
  ;[1 0 0] Event to update clues for escape
  (Variables|/Game/Systems/UI_HUD/W_PlayerHUD_UI.W_PlayerHUD_UI_C|SetCluesFound_Text _w_updateclue_ref (Utilities|Text|ToText(Integer) CluesFound))
  (Class|EditableTextBox|SetForegroundColor _cluesfound_cluecount "(R=0.000000,G=0.750000,B=0.063900,A=1.000000)")
  (Utilities|FlowControl|Delay 0.7)
  (Class|EditableTextBox|SetForegroundColor _cluesfound_cluecount "(R=1.000000,G=1.000000,B=1.000000,A=1.000000)"))

(event Custom|Reset_DamageTaken)

(event Custom|Enter_ResetDamageTaken
  ;[0.04638 0.2073 1] BEGIN PLAY
  ;;[0 0 0] Player taking damage bind event on begin play
  (Utilities|FlowControl|DoOnce false) ; enters at Reset
)

(event Custom|OnTakeAnyDamage_Enter
  (params (DamagedActor :type Actor%20Object%20Reference) (Damage :type Float%20%28single-precision%29) (DamageType :type Damage%20Type%20Object%20Reference) (InstigatedBy :type Controller%20Object%20Reference) (DamageCauser :type Actor%20Object%20Reference))
  ;[0.04638 0.2073 1] BEGIN PLAY
  ;;[0 0 0] Player taking damage bind event on begin play
  (Utilities|FlowControl|DoOnce false
    (:Completed
      (if (!= (Variables|Components|GetPlayer_CurHealth) 0.0)
        (bind _output_get (Variables|Components|SetPlayer_CurHealth (- (Variables|Components|GetPlayer_CurHealth) Damage)))
        (CallFunction|UpdateHealth _output_get)
        (CallFunction|FBloodonScreen)
        (CallFunction|EnterResetDamageTaken)
        (else
          (Variables|Default|SetRespawn_Transform (Transformation|GetActorTransform self))
          (Variables|/Game/Character/AnimStarterPack/UE4ASP_HeroTPP_AnimBlueprint.UE4ASP_HeroTPP_AnimBlueprint_C|SetbIsDead? (Variables|Components|GetAnim%20BP%20Ref) true)
          (Utilities|FlowControl|Delay 5.0)
          (Actor|DestroyActor))))))

(event EventBeginPlay
  (bind (_playerchar_ref _playercontrol_ref _animbp_ref) (CallFunction|GetPlayerCharacterP))
  ;[0.04638 0.2073 1] BEGIN PLAY
  ;;[0.01042 0.01042 0.01042] Saving Controller as ObjRef
  (Variables|Components|SetPlayer%20Control%20Ref _playercontrol_ref)
  ;;[0.01042 0.01042 0.01042] Saving Anim BP as ObjRef
  (Variables|Components|SetAnim%20BP%20Ref _animbp_ref)
  ;;[0.01562 0.01562 0.01562] Adding Player HUD/UI to viewport
  (bind _returnvalue (UserInterface|CreateWidget "/Game/Systems/UI_HUD/W_PlayerHUD_UI.W_PlayerHUD_UI_C"))
  (bind _output_get (Variables|Default|SetW_UpdateClue_Ref _returnvalue))
  (Widget|SetVisibility (Variables|/Game/Systems/UI_HUD/W_PlayerHUD_UI.W_PlayerHUD_UI_C|GetInteract_Text _output_get) (Variables|Default|GetInteractText_SetHidden))
  (UserInterface|Viewport|AddtoViewport _output_get 0)
  (CallFunction|UpdateHealth (Variables|Components|GetPlayer_CurHealth))
  ;;[0 0 0] Door Puzzle piece control
  (Variables|Default|SetbHasCone false)
  (Variables|Default|SetbHasSphere false)
  (Variables|Default|SetbHasCube false)
  ;;[0 0.07173 0.151] Binding: TakeAnyDamage from BEGIN PLAY
  (EventDispatchers|AssignOnTakeAnyDamage (delegate Custom|OnTakeAnyDamage_Enter)))

(event EventTick
  (params (DeltaSeconds :type Float%20%28single-precision%29))
  ;[1 0 0] PER FRAME EVENTS
  ;;[0 0 0] Object interaction line trace
  (CallFunction|SeekingInteractable))

(event Input|ActionEvents|InputActionInteract
  (params (Key :type Key%20Structure :default "None"))
  ;[0.01531 0.151 0.02574] Press "E" To Interact
  (:Pressed
    (Utilities|FlowControl|Sequence
      (:then_0
        (bind _interactable (Variables|Default|GetInteractable)
          (:then
            (Class|IInteract|Interact(Message) _interactable))
          (:else
            (Variables|Default|SetInteractable 0)))))))

(event Input|ActionEvents|InputActionFlashlight
  (params (Key :type Key%20Structure :default "None"))
  (bind _light (Variables|Default|GetLight))
  ;[0.125 0.09834 0] Turn flashlight on or of be pressing "F"
  (:Pressed
    (Utilities|FlowControl|FlipFlop
      (:A
        (Rendering|SetVisibility _light false false))
      (:B
        (Rendering|SetVisibility _light true false)))))

(fn ConstructionScript)

(fn SeekingInteractable
  (bind _followcamera (Variables|Camera|GetFollowCamera))
  (bind _returnvalue (Transformation|GetWorldLocation _followcamera))
  ;[0.6037 0.1874 1] Line tracing seeking interactables in the player's environment
  (bind _outhit (Collision|LineTraceByChannel _returnvalue (+ (* (Math|Vector|GetForwardVector (Transformation|GetWorldRotation _followcamera)) 2e+02) _returnvalue) "TraceTypeQuery3" false (Utilities|Array|MakeArray self) "None" true "(R=0.030084,G=1.000000,B=0.000000,A=1.000000)" "(R=1.000000,G=0.000000,B=0.009744,A=1.000000)"))
  (Utilities|IsValid (.HitActor (Collision|BreakHitResult _outhit))
    (:Is%20Valid
      (if (and (.bBlockingHit (Collision|BreakHitResult _outhit)) (or (Actor|ActorHasTag (.HitActor (Collision|BreakHitResult _outhit)) "Interactable") (Components|ComponentHasTag (.HitComponent (Collision|BreakHitResult _outhit)) "Interactable")))
        (Widget|SetVisibility (Variables|/Game/Systems/UI_HUD/W_PlayerHUD_UI.W_PlayerHUD_UI_C|GetInteract_Text (Variables|Default|GetW_UpdateClue_Ref)) "Visible")
        (CallFunction|SetInteractObject (.HitActor (Collision|BreakHitResult _outhit)))
        (Utilities|IsValid (.HitComponent (Collision|BreakHitResult _outhit))
          (:Is%20Valid
            (CallFunction|SetInteractObject (Components|GetOwner (.HitComponent (Collision|BreakHitResult _outhit))))
            (if (Components|ComponentHasTag (.HitComponent (Collision|BreakHitResult _outhit)) "Cone")
              (Variables|Default|SetbHasCone true)
              (elif (Components|ComponentHasTag (.HitComponent (Collision|BreakHitResult _outhit)) "Sphere")
                (Variables|Default|SetbHasSphere true)
                (elif (Components|ComponentHasTag (.HitComponent (Collision|BreakHitResult _outhit)) "Cube")
                  (Variables|Default|SetbHasCube true)))))
          (:Is%20Not%20Valid
            (Variables|Default|SetInteractable 0)
            (Widget|SetVisibility (Variables|/Game/Systems/UI_HUD/W_PlayerHUD_UI.W_PlayerHUD_UI_C|GetInteract_Text (Variables|Default|GetW_UpdateClue_Ref)) (Variables|Default|GetInteractText_SetHidden))))
        (else
          (Variables|Default|SetInteractable 0 :!label _label)
          (Widget|SetVisibility (Variables|/Game/Systems/UI_HUD/W_PlayerHUD_UI.W_PlayerHUD_UI_C|GetInteract_Text (Variables|Default|GetW_UpdateClue_Ref)) (Variables|Default|GetInteractText_SetHidden)))))
    (:Is%20Not%20Valid
      (goto _label))))

(fn UpdateHealth
  (params (Current_PlayerHealth :type Float%20%28double-precision%29))
  (Progress|SetPercent (Variables|/Game/Systems/UI_HUD/W_PlayerHUD_UI.W_PlayerHUD_UI_C|GetHUD_PlayerHealth (Variables|Default|GetW_UpdateClue_Ref)) (/ Current_PlayerHealth 1e+02)))

(fn SetInteractObject
  (params (NewParam :type Actor%20Object%20Reference))
  ;[0.6083 0.1768 1] Once the line trace deems an object as interactable (Actor Has Tag: Interactable) this function will set the Interactable object reference tothe "HitActor"
  (if (!= NewParam 0)
    (bind _output_get (Variables|Default|SetInteractable NewParam))
    (return _output_get)
    (else
      (Widget|SetVisibility (Variables|/Game/Systems/UI_HUD/W_PlayerHUD_UI.W_PlayerHUD_UI_C|GetInteract_Text (Variables|Default|GetW_UpdateClue_Ref)) (Variables|Default|GetInteractText_SetHidden)))))

(fn FNotifySound
  ;[0.08734 0 0.1927] When the player steps can be heard by enemies
  (Class|AudioLinkBlueprintInterface|SetLinkSound(Message) (Variables|Default|GetAIPerceptionStimuliSource) "/Game/Character/FPS_AnimBP_v2/Audio/Footsteps/Concrete/WAV/WAV_Footstep_Concrete_Walk01.WAV_Footstep_Concrete_Walk01"))

(fn FBloodonScreen
  ;[0.03045 0.001276 0.06771] Displaying blood on screen widget when the player gets hit and takes damage.
  (Variables|Camera|GetW_PlayerHurtFX_Ref
    (:then
      (Default|EnterPlayHitAnim (Variables|Camera|GetW_PlayerHurtFX_Ref)))
    (:else
      (bind _returnvalue (UserInterface|CreateWidget "/Game/Systems/UI_HUD/w_PlayerHurtFX.w_PlayerHurtFX_C" (Variables|Components|GetPlayer%20Control%20Ref)))
      (bind _output_get (Variables|Camera|SetW_PlayerHurtFX_Ref _returnvalue))
      (UserInterface|Viewport|AddtoViewport _output_get 0))))