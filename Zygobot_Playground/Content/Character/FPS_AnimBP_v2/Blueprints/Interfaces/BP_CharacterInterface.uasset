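; Blueprint interface for the first-person character, letting animation, weapons, pickups and settings talk to it without casting.
; Getters expose movement state, camera transform and curve values, hand IK, aim, recoil, near-wall distance, weapon data and reserve ammo.
; Commands and notifies cover equip, reload, grenade spawning, receiving weapons, attachments and ammo, applying settings, and restoring inventory on spawn.
; It declares signatures only; implementers supply the behaviour.
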(fn GetMovementStateValues
  (return "NewEnumerator0" "NewEnumerator0" 0.0 0.0 0.0 0.0 0.0 0.0 0.0 false))

(fn GetCameraLocationandRotation
  (return "0, 0, 0" "0, 0, 0"))

(fn OnFinishUnequip)

(fn GetHandIKTransforms
  (return "" ""))

(fn GetWeaponData
  (params (EquippedWeapon :type Boolean) (Index :type Integer))
  (return "" false))

(fn ReloadAmmo)

(fn SpawnGrenade)

(fn RecieveWeapon
  (params (NewWeapon :type Boolean) (Weapon%20Data :type ST%20Gun%20Data%20Structure))
  (return false))

(fn StartReloadWeapon)

(fn GetIsAiming
  (return false))

(fn RecieveWeaponAttachment
  (params (Attachment%20Data%20Asset :type FPS%20PDA%20Attachment%20Data%20Base%20Object%20Reference))
  (return false))

(fn RecieveAmmo
  (params (AmmoDataAsset :type FPS%20PDA%20Ammo%20Data%20Base%20Object%20Reference) (AmmoAmountOverride :type Integer))
  (return false))

(fn SetSettings
  (params (Settings :type ST%20Settings%20Structure)))

(fn UpdateFloatSetting
  (params (Setting :type E_Settings%20Enum :default "NewEnumerator0") (Value :type Float%20%28single-precision%29)))

(fn UpdateBoolSetting
  (params (Setting :type E_Settings%20Enum :default "NewEnumerator0") (Value :type Boolean)))

(fn RestoreWeaponInventoryonSpawn
  (params (Inventory :type Array%20of%20BP%20Weapon%20Base%20Object%20References) (Active%20Equipped%20Index :type Integer)))

(fn GetCameraCurveValues
  (return 0.0 0.0 0.0 "0, 0, 0" 0.0))

(fn GetCameraRotationDelta
  (return "0, 0, 0" "0, 0, 0"))

(fn OnFinishEquipWeapon)

(fn GetNearWallDistance
  (return 0.0))

(fn GetRecoilScalar
  (return 0.0))

(fn GetCurrentReserveAmmo
  (params (Ammo%20Data%20Asset :type FPS%20PDA%20Ammo%20Data%20Base%20Object%20Reference))
  (return 0))