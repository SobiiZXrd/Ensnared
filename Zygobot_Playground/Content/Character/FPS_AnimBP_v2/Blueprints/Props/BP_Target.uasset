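; Shooting-range target actor that drops when shot, awards zone-based points and pops back up after a delay.
; Point damage is matched against an ordered list of head and body hit components, whose index selects score, headshot flag and text colour.
; Hits fire the OnTargetHit dispatcher and print the score.
; Timelines rotate the mesh down and, via a timer, back up, with an IsHit flag blocking repeat hits until reset.
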(event Custom|ResetTarget
  ;[0 0 0] The timer that starts after the target has lowered calls this event when it elapses. Start raising the target back up
  (Components|Timeline|PlayfromStart (Variables|Default|GetTL_Reset)))

(event Custom|OnTargetReset
  ;[0 0 0] When the target has returned to its default position, allow it to be hit again
  (Variables|Default|SetIsHit false))

(event Custom|OnHIt
  (params (Is%20Headshot :type Boolean) (Score :type Float%20%28single-precision%29) (TextColor :type Linear%20Color%20Structure))
  ;[0 0 0] Print some score on hit for fun
  (Default|CallOnTargetHit Is%20Headshot Score)
  (Development|PrintString (Utilities|String|Append (select Is%20Headshot "Headshot! " "") (Utilities|String|ToString(Text) (Utilities|Text|ToText(Float) Score "HalfToEven" false true 1 324 0 1)) " Points!") true false TextColor 1e+01))

(event EventBeginPlay
  ;[0 0 0] Give the target a little animation to start
  (CallFunction|SetTargetAreas)
  (CallFunction|ResetTarget))

(event Game|Damage|EventPointDamage
  (params (Damage :type Float%20%28single-precision%29) (DamageType :type Damage%20Type%20Object%20Reference) (HitLocation :type Vector :default "0, 0, 0") (HitNormal :type Vector :default "0, 0, 0") (HitComponent :type Primitive%20Component%20Object%20Reference) (BoneName :type Name :default "None") (ShotFromDirection :type Vector :default "0, 0, 0") (InstigatedBy :type Controller%20Object%20Reference) (DamageCauser :type Actor%20Object%20Reference) (HitInfo :type Hit%20Result%20Structure%20%28by%20ref%29))
  ;[0 0 0] If the target has not already been hit since resetting, start lowering it
  (if (not (Variables|Default|GetIsHit))
    (Variables|Default|SetIsHit true)
    (Components|Timeline|PlayfromStart (Variables|Default|GetTL_OnHit))
    (bind (_index_found _index) (CallFunction|FindHitComponentIndex HitComponent))
    (if _index_found
      (CallFunction|OnHIt (.IsHeadshot (CallFunction|GetScore _index)) (.Score (CallFunction|GetScore _index)) (.Colour (CallFunction|GetScore _index))))))

(fn ConstructionScript)

(fn SetTargetAreas
  (bind _targetcomponentslist (Variables|Default|GetTargetComponentsList))
  (Utilities|Array|Add _targetcomponentslist (Variables|Default|GetHeadTarget0))
  (Utilities|Array|Add _targetcomponentslist (Variables|Default|GetHeadTarget1))
  (Utilities|Array|Add _targetcomponentslist (Variables|Default|GetHeadTarget2))
  (Utilities|Array|Add _targetcomponentslist (Variables|Default|GetHeadTarget3))
  (Utilities|Array|Add _targetcomponentslist (Variables|Default|GetBodyTarget0))
  (Utilities|Array|Add _targetcomponentslist (Variables|Default|GetBodyTarget1))
  (Utilities|Array|Add _targetcomponentslist (Variables|Default|GetBodyTarget2))
  (Utilities|Array|Add _targetcomponentslist (Variables|Default|GetBodyTarget3))
  (Utilities|Array|Add _targetcomponentslist (Variables|Default|GetBodyTarget4)))

(fn FindHitComponentIndex
  (params (ItemToFind :type Primitive%20Component%20Object%20Reference%20%28by%20ref%29))
  (bind _targetcomponentslist (Variables|Default|GetTargetComponentsList))
  (bind _returnvalue (Utilities|Array|FindItem _targetcomponentslist ItemToFind))
  (return (>= _returnvalue 0) _returnvalue))

(fn GetScore
  (params (Component%20Index :type Integer))
  ;[0 0 0] 0-4 is headshots, 5-9 is body
  (return (and (>= Component%20Index 0) (<= Component%20Index 3)) (Utilities|Select :Index Component%20Index :Option%200 7.0 :Option%201 8.0 :Option%202 9.0 :Option%203 15.0 :Option%204 7.0 :Option%205 8.0 :Option%206 9.0 :Option%207 1e+01 :Option%208 12.0) (Utilities|Select :Index Component%20Index :Option%200 "(R=1.000000,G=0.902361,B=0.000000,A=1.000000)" :Option%201 "(R=1.000000,G=0.506319,B=0.000000,A=1.000000)" :Option%202 "(R=1.000000,G=0.279171,B=0.000000,A=1.000000)" :Option%203 "(R=1.000000,G=0.007639,B=0.000000,A=1.000000)" :Option%204 "(R=0.000000,G=0.278582,B=1.000000,A=1.000000)" :Option%205 "(R=0.000000,G=0.702252,B=1.000000,A=1.000000)" :Option%206 "(R=0.000000,G=0.944436,B=1.000000,A=1.000000)" :Option%207 "(R=0.000000,G=1.000000,B=0.389239,A=1.000000)" :Option%208 "(R=0.000000,G=1.000000,B=0.020782,A=1.000000)")))

(fn DestroySelf
  (Actor|DestroyActor))