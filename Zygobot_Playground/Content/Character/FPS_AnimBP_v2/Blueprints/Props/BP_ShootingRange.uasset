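; BP_ShootingRange is a shooting range actor that spawns BP_Target actors in rows across a configurable box area.
; SpawnAllTargets clears existing targets, then spaces each row's count from TargetRows evenly across the box.
; A downward visibility trace sets each target's height on the surface below before it attaches to the box.
; A DestroyAllTargets dispatcher clears targets on respawn or destruction; the target-hit handler is empty.
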(event EventBeginPlay)

(event Collision|EventActorBeginOverlap
  (params (OtherActor :type Actor%20Object%20Reference)))

(event EventTick
  (params (DeltaSeconds :type Float%20%28single-precision%29)))

(event EventDestroyed
  (CallFunction|RemoveAllTargets))

(fn ConstructionScript
  (bind _box (Variables|Default|GetBox))
  (Transformation|SetRelativeLocation _box (Variables|Default|GetLocation) false false)
  (Components|Box|SetBoxExtent _box (Variables|Default|GetSpawnArea) true))

(fn SpawnTarget
  (params (Spawn%20Transform :type Transform))
  (bind _returnvalue (Game|SpawnActorfromClass "/Game/FPS_AnimBP_v2/Blueprints/Props/BP_Target.BP_Target_C" (Math|Transform|MakeTransform "0, 0, 0" "0, 0, 0" "1,1,1") "AdjustIfPossibleButAlwaysSpawn" 0 0))
  (EventDispatchers|BindEventtoOnTargetHit _returnvalue (EventDispatchers|CreateEvent :!event OnTargetHit))
  (EventDispatchers|BindEventtoDestroyAllTargets (EventDispatchers|CreateEvent _returnvalue :!event DestroySelf))
  (Transformation|AttachComponentToComponent _returnvalue (Variables|Default|GetBox) "None" "SnapToTarget" "SnapToTarget" "KeepRelative" true)
  (Transformation|SetRelativeTransform (Variables|/Game/FPS_AnimBP_v2/Blueprints/Props/BP_Target.BP_Target_C|GetDefaultSceneRoot _returnvalue) Spawn%20Transform false false)
  (Math|Integer|IncrementInt (Variables|Default|GetTotalTargets)))

(fn SpawnAllTargets
  (CallFunction|RemoveAllTargets)
  (LocalVariables|Setlocal_NumberOfRows (Utilities|Array|LastIndex (Variables|Default|GetTargetRows)))
  (for (_array_element _array_index) (Variables|Default|GetTargetRows)
    (bind _output_get (LocalVariables|Setlocal_TargetsThisRow (- _array_element 1)))
    (LocalVariables|Setlocal_CurrentRow _array_index)
    (for _index (range 0 _output_get)
      (LocalVariables|Setlocal_CurrentTargetThisRow _index)
      (bind _spawn_transform (CallFunction|CalculateSpawnLocation (LocalVariables|Getlocal_NumberOfRows) (LocalVariables|Getlocal_CurrentRow) (LocalVariables|Getlocal_TargetsThisRow) (LocalVariables|Getlocal_CurrentTargetThisRow)))
      (CallFunction|SpawnTarget _spawn_transform))))

(fn OnTargetHit
  (params (IsHeadshot :type Boolean) (Score :type Float%20%28single-precision%29)))

(fn RemoveAllTargets
  (Default|CallDestroyAllTargets)
  (Variables|Default|SetTotalTargets 0))

(fn CalculateSpawnLocation
  (params (Number%20of%20Rows :type Integer) (Current%20Row :type Integer) (Targets%20This%20Row :type Integer) (Current%20Target%20This%20%20Row :type Integer))
  (bind _box (Variables|Default|GetBox))
  (bind _spawnarea (Variables|Default|GetSpawnArea))
  (bind _spawnarea_2 (Variables|Default|GetSpawnArea))
  (bind _spawnarea_3 (Variables|Default|GetSpawnArea))
  (bind _returnvalue (Transformation|GetWorldTransform _box))
  (Utilities|FlowControl|Sequence
    (:then_0
      (LocalVariables|Setlocal_SpawnX (- (* (/ (* (.x _spawnarea_3) 2.0) (Math|Conversions|ToFloat(Integer) Number%20of%20Rows)) (Math|Conversions|ToFloat(Integer) Current%20Row)) (.x _spawnarea_3)))
      (LocalVariables|Setlocal_SpawnY (- (* (/ (* (.y _spawnarea_2) 2.0) (Math|Conversions|ToFloat(Integer) Targets%20This%20Row)) (Math|Conversions|ToFloat(Integer) Current%20Target%20This%20%20Row)) (.y _spawnarea_2))))
    (:then_1
      (bind (_outhit _returnvalue_2) (Collision|LineTraceByChannel (+ (.location _returnvalue) (* (Math|Vector|GetForwardVector (.rotation _returnvalue)) (LocalVariables|Getlocal_SpawnX)) (* (Math|Vector|GetRightVector (.rotation _returnvalue)) (LocalVariables|Getlocal_SpawnY)) (Math|Vector|MakeVector 0.0 0.0 (.z _spawnarea))) (+ (+ (.location _returnvalue) (* (Math|Vector|GetForwardVector (.rotation _returnvalue)) (LocalVariables|Getlocal_SpawnX)) (* (Math|Vector|GetRightVector (.rotation _returnvalue)) (LocalVariables|Getlocal_SpawnY)) (Math|Vector|MakeVector 0.0 0.0 (.z _spawnarea))) (Math|Vector|MakeVector 0.0 0.0 (* (.z _spawnarea) -2.0))) "TraceTypeQuery1" false 0 "None"))
      (if _returnvalue_2
        (LocalVariables|Setlocal_SpawnZ (- (.Z (Math|Vector|BreakVector (.ImpactPoint (Collision|BreakHitResult _outhit)))) (.z (Transformation|GetWorldLocation (Variables|Default|GetBox)))))
        (else
          (LocalVariables|Setlocal_SpawnZ 0.0))))
    (:then_2
      (return (Math|Transform|MakeTransform (Math|Vector|MakeVector (LocalVariables|Getlocal_SpawnX) (LocalVariables|Getlocal_SpawnY) (LocalVariables|Getlocal_SpawnZ)) (Variables|Default|GetTargetRotation) "1,1,1")))))