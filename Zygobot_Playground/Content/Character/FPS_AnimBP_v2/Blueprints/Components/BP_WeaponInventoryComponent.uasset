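; Player inventory component for an FPS that holds a fixed number of spawned weapon actors, unlocked attachments and reserve ammo per ammo data asset.
; New weapons fill empty slots or replace the active one, which drops as a physics pickup.
; Switching records a target index, applied separately on equip, with cycling and holstering supported.
; Weapons are snapshotted as gun data to respawn them after death or a save load.
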(event EventBeginPlay
  ;[0 0 0] Initialise the inventory component on creation
  (General|InitializeInventory))

(fn TryRecieveWeapon
  (params (Is%20New%20Weapon :type Boolean) (Weapon%20Data :type ST%20Gun%20Data%20Structure))
  (bind _activeequippedweaponindex (Variables|LiveData|GetActiveEquippedWeaponIndex))
  ;[0 0 0] Try to recieve a new weapon. If there's space, add it to the inventory. If not, drop the current weapon first
  (for (_array_element _array_index) (Variables|LiveData|GetEquippedWeapons)
    (Utilities|IsValid _array_element
      (:Is%20Not%20Valid
        (Weapon|SpawnandAddEquippedWeapon Weapon%20Data _array_index Is%20New%20Weapon)
        (return true))))
  (Weapon|DropWeapon _activeequippedweaponindex false)
  (Weapon|SpawnandAddEquippedWeapon Weapon%20Data _activeequippedweaponindex Is%20New%20Weapon)
  (return true))

(fn SpawnandAddEquippedWeapon
  (params (Weapon%20Data :type ST%20Gun%20Data%20Structure) (Index%20To%20Equip :type Integer) (Is%20New%20Weapon :type Boolean))
  (bind _spawned_weapon (Weapon|SpawnWeapon Weapon%20Data Index%20To%20Equip Is%20New%20Weapon))
  (LocalVariables|Setlocal_SpawnedWeapon _spawned_weapon)
  (Utilities|FlowControl|Sequence
    (:then_0
      ;[0 0 0] Equip all the attachments specified in the Attachments list.
      (Attachments|EquipAllCurrentAttachmentsonWeapon (LocalVariables|Getlocal_SpawnedWeapon)))
    (:then_1
      ;[0 0 0] Either equip or hide the weapon based on the current index
      (if (== (Variables|LiveData|GetActiveEquippedWeaponIndex) Index%20To%20Equip)
        (Weapon|EquipActiveWeapon Index%20To%20Equip :!label _label)
        (else
          (Utilities|IsWeaponValid (Variables|LiveData|GetActiveEquippedWeaponIndex)
            (:Is%20Valid
              (Default|SetIsActiveWeapon (LocalVariables|Getlocal_SpawnedWeapon) false))
            (:Is%20Not%20Valid
              (goto _label))))))))

(fn SpawnWeapon
  (params (Weapon%20Data :type ST%20Gun%20Data%20Structure%20%28by%20ref%29) (IndexToEquip :type Integer) (Is%20New%20Weapon :type Boolean))
  (bind _returnvalue (Game|GetPlayerCharacter 0))
  ;[0 0 0] Spawn the weapon and add the reference to the live weapon inventory
  (bind _returnvalue_2 (Game|SpawnActorfromClass (Variables|/Game/FPS_AnimBP_v2/Blueprints/DataAssets/Weapons/Guns/FPS_PDA_GunBase.FPS_PDA_GunBase_C|GetGunClass (Utilities|Struct|BreakST_GunData Weapon%20Data)) (Transformation|GetWorldTransform (Variables|/Script/Engine.Actor|GetRootComponent _returnvalue)) "AlwaysSpawn" _returnvalue (Variables|Default|GetOwningController) Is%20New%20Weapon _returnvalue))
  (Utilities|IsValid _returnvalue_2
    (:Is%20Valid
      (bind _output_get (LocalVariables|Setlocal_SpawnedWeapon _returnvalue_2))
      (Default|InitialiseGun _output_get Weapon%20Data)
      (Utilities|Array|SetArrayElem (Variables|LiveData|GetEquippedWeapons) IndexToEquip (LocalVariables|Getlocal_SpawnedWeapon))
      (Default|CallOnWeaponSpawned (LocalVariables|Getlocal_SpawnedWeapon))
      (return (LocalVariables|Getlocal_SpawnedWeapon)))))

(fn DropWeapon
  (params (Index%20to%20Drop :type Integer) (CycleToNext :type Boolean))
  ;[0 0 0] Drop the current weapon, remove it from the inventory and create a pickup for it.
  (bind _weapon (Utilities|GetWeaponatIndex Index%20to%20Drop)
    (:Is%20Valid
      (bind _output_get (LocalVariables|Setlocal_Weapon _weapon))
      (LocalVariables|Setlocal_WeaponData (Default|GetGunData _output_get))
      (bind (_location _rotation) (Class|BPCharacterInterface|GetCameraLocationandRotation(Message) (Game|GetPlayerCharacter 0)))
      (bind _returnvalue (Game|SpawnActorfromClass "/Game/FPS_AnimBP_v2/Blueprints/Pickups/BP_PickupGun.BP_PickupGun_C" (Math|Transform|MakeTransform (+ _location (* (Math|Vector|GetForwardVector _rotation) 8e+01)) _rotation "1,1,1") "Undefined" 0 false (LocalVariables|Getlocal_WeaponData) (Utilities|Struct|BreakST_GunData (LocalVariables|Getlocal_WeaponData)) true false 0.0 "(R=1.000000,G=1.000000,B=1.000000,A=1.000000)" 0))
      (Physics|AddImpulse (Variables|/Game/FPS_AnimBP_v2/Blueprints/Pickups/BP_PickupBase.BP_PickupBase_C|GetSkeletalMesh _returnvalue) (* (Math|Vector|GetForwardVector _rotation) 5e+02) "None" true)
      (Default|CallOnDropWeapon CycleToNext)
      (Actor|DestroyActor (LocalVariables|Getlocal_Weapon))
      (Utilities|Array|SetArrayElem (Variables|LiveData|GetEquippedWeapons) Index%20to%20Drop 0))))

(fn EquipActiveWeapon
  (params (Index%20To%20Equip :type Integer))
  (bind (_is_valid _weapon) (Weapon|GetActiveEquippedWeapon))
  ;[0 0 0] Make sure the weapon being equipped is valid. If a weapon is already equipped, hide it.
  (Utilities|IsWeaponValid Index%20To%20Equip
    (:Is%20Valid
      (Variables|LiveData|SetWeaponIsHolstered false)
      (if _is_valid
        (Default|SetIsActiveWeapon _weapon false))
      ;[0 0 0] Set the active weapon
      (bind _output_get (Variables|LiveData|SetActiveEquippedWeaponIndex Index%20To%20Equip))
      (Variables|LiveData|SetWeaponSwitchToIndex _output_get)
      (bind _output_get_2 (LocalVariables|Setlocal_Weapon (.Weapon (Weapon|GetActiveEquippedWeapon))))
      (Default|SetIsActiveWeapon _output_get_2 true)
      (Default|CallOnEquipActiveWeapon _output_get_2))))

(fn GetActiveEquippedWeapon
  ;[0 0 0] Get the currently equipped weapon if one exists
  (if (not (Variables|LiveData|GetWeaponIsHolstered))
    (bind _weapon (Utilities|GetWeaponatIndex (Variables|LiveData|GetActiveEquippedWeaponIndex))
      (:Is%20Valid
        (return true _weapon))
      (:Is%20Not%20Valid
        _)))
  (return false 0))

(fn GetWeaponInventory
  (return (Variables|LiveData|GetEquippedWeapons)))

(fn CycleWeapon
  (params (ToNextWeapon :type Boolean))
  ;[0 0 0] Cycle through the weapon inventory, either forwards or backwards based on the bool input, and find the first valid weapon to switch to. Don't switch if only one weapon is present
  (LocalVariables|Setlocal_CurrentIndex (Variables|LiveData|GetActiveEquippedWeaponIndex))
  (bind _output_get (LocalVariables|Setlocal_LastIndex (Utilities|Array|LastIndex (Variables|LiveData|GetEquippedWeapons))))
  (Utilities|FlowControl|ForLoopwithBreak 0 _output_get :!label _label
    (:LoopBody
      (Utilities|FlowControl|Sequence
        (:then_0
          (if ToNextWeapon
            (if (== (LocalVariables|Getlocal_CurrentIndex) (LocalVariables|Getlocal_LastIndex))
              (LocalVariables|Setlocal_SwitchToIndex 0)
              (else
                (bind _result (Math|Integer|IncrementInt (LocalVariables|Getlocal_CurrentIndex))
                  (:%20%20
                    (LocalVariables|Setlocal_SwitchToIndex _result)))))
            (elif (== (LocalVariables|Getlocal_CurrentIndex) 0)
              (LocalVariables|Setlocal_SwitchToIndex (LocalVariables|Getlocal_LastIndex))
              (else
                (bind _result_2 (Math|Integer|DecrementInt (LocalVariables|Getlocal_CurrentIndex))
                  (:%20%20
                    (LocalVariables|Setlocal_SwitchToIndex _result_2)))))))
        (:then_1
          (Utilities|IsWeaponValid (LocalVariables|Getlocal_SwitchToIndex)
            (:Is%20Valid
              (LocalVariables|Setlocal_IsValidIndex true)
              (goto _label Break))
            (:Is%20Not%20Valid
              (LocalVariables|Setlocal_IsValidIndex false)
              (LocalVariables|Setlocal_CurrentIndex (LocalVariables|Getlocal_SwitchToIndex)))))))
    (:Completed
      (if (and (LocalVariables|Getlocal_IsValidIndex) (!= (Variables|LiveData|GetActiveEquippedWeaponIndex) (LocalVariables|Getlocal_SwitchToIndex)))
        (Variables|LiveData|SetWeaponSwitchToIndex (LocalVariables|Getlocal_SwitchToIndex))
        (return true)
        (else
          (return false))))))

(fn GetActiveEquippedWeaponIndex
  (return (Variables|LiveData|GetActiveEquippedWeaponIndex)))

(fn GetWeaponData
  (params (Equipped%20Weapon :type Boolean) (Index :type Integer))
  (bind _weapon (Weapon|GetActiveEquippedWeapon))
  ;[0 0 0] Send the data on the currently equipped weapon
  (if Equipped%20Weapon
    (Utilities|IsValid _weapon
      (:Is%20Valid
        (return (Default|GetGunData _weapon) true))
      (:Is%20Not%20Valid
        _))
    (else
      (bind _weapon_2 (Utilities|GetWeaponatIndex Index)
        (:Is%20Valid
          (return (Default|GetGunData _weapon_2) true))
        (:Is%20Not%20Valid
          _))))
  (return "" false))

(fn GetWeaponSwitchtoIndex
  (return (Variables|LiveData|GetWeaponSwitchToIndex)))

(fn SetSwitchtoIndex
  (params (SwitchToIndex :type Integer))
  ;[0 0 0] Set the index you want to switch to before actually attempting to switch weapon
  (if (or (!= SwitchToIndex (Variables|LiveData|GetWeaponSwitchToIndex)) (Variables|LiveData|GetWeaponIsHolstered))
    (Utilities|IsWeaponValid SwitchToIndex
      (:Is%20Valid
        (Variables|LiveData|SetWeaponSwitchToIndex SwitchToIndex)
        (return true))
      (:Is%20Not%20Valid
        _)))
  (return false))

(fn RestoreFullInventory
  (params (Inventory%20Data :type Array%20of%20ST%20Gun%20Data%20Structures) (ActiveEquippedWeaponIndex :type Integer))
  ;[0 0 0] Restore the full weapon inventory from a Gun Data array
  (for (_array_element _array_index) Inventory%20Data
    (if (Utilities|Enum|NotEqual(Enum) (Variables|/Game/FPS_AnimBP_v2/Blueprints/DataAssets/Weapons/FPS_PDA_WeaponBase.FPS_PDA_WeaponBase_C|GetWeaponType (Utilities|Struct|BreakST_GunData _array_element)) "NewEnumerator0")
      (bind _spawned_weapon (Weapon|SpawnWeapon _array_element _array_index false))
      (Rendering|SetActorHiddenInGame _spawned_weapon true)
      (Attachments|EquipAllCurrentAttachmentsonWeapon _spawned_weapon)))
  (bind _output_get (Variables|LiveData|SetActiveEquippedWeaponIndex ActiveEquippedWeaponIndex))
  (Weapon|SetSwitchtoIndex _output_get)
  (Weapon|EquipActiveWeapon (Variables|LiveData|GetActiveEquippedWeaponIndex)))

(fn GetWeaponInventoryData
  ;[0 0 0] Get the weapon inventory in the form of Gun Data rather than hard actor references
  (for (_array_element _array_index) (Variables|LiveData|GetEquippedWeapons)
    (Utilities|IsValid _array_element
      (:Is%20Valid
        (Utilities|Array|SetArrayElem (LocalVariables|Getlocal_InventoryData) _array_index (Default|GetGunData _array_element) true))))
  (return (LocalVariables|Getlocal_InventoryData)))

(fn DestroyWeaponActors
  ;[0 0 0] Destroy all spawned weapons
  (for _array_element (Variables|LiveData|GetEquippedWeapons)
    (Utilities|IsValid _array_element
      (:Is%20Valid
        (Actor|DestroyActor _array_element)))))

(fn TryRecieveAttachment
  (params (Attachment%20Data%20Asset :type FPS%20PDA%20Attachment%20Data%20Base%20Object%20Reference) (Equip%20Attachment :type Boolean))
  ;[0 0 0] Try to recieve an attachment to add to the inventory. Fails if the attachment is already contained in the inventory
  (Utilities|IsValid Attachment%20Data%20Asset
    (:Is%20Valid
      (if (not (Utilities|Array|ContainsItem (Variables|LiveData|GetAttachmentAssetsInventory) Attachment%20Data%20Asset))
        (Utilities|Array|AddUnique (Variables|LiveData|GetAttachmentAssetsInventory) Attachment%20Data%20Asset)
        (return true)
        (else
          _)))
    (:Is%20Not%20Valid
      _))
  (return false))

(fn EquipWeaponAttachment
  (params (Weapon :type BP%20Weapon%20Base%20Object%20Reference) (Attachment%20Data%20Asset :type FPS%20PDA%20Attachment%20Data%20Base%20Object%20Reference))
  ;[0 0 0] Equip an attachment to the weapon, and add it to the attachments inventory if it is not already there
  (Utilities|FlowControl|Sequence
    (:then_0
      (bind _attachment_data_asset (LocalVariables|GetAttachment%20Data%20Asset)
        (:then
          (if (Variables|/Game/FPS_AnimBP_v2/Blueprints/DataAssets/Attachments/FPS_PDA_AttachmentDataBase.FPS_PDA_AttachmentDataBase_C|GetAttachmentCanBeAddedToInventory _attachment_data_asset)
            (Attachments|TryRecieveAttachment _attachment_data_asset false)))
        (:else)))
    (:then_1
      (bind _weapon (LocalVariables|GetWeapon)
        (:then
          (bind _success (Default|EquipAttachment _weapon Attachment%20Data%20Asset))
          (return _success))
        (:else)))))

(fn CancelUnequip
  ;[0 0 0] Set the Switch to Index back to the current index if the equip was cancelled
  (Variables|LiveData|SetWeaponSwitchToIndex (Variables|LiveData|GetActiveEquippedWeaponIndex)))

(fn CanReloadCheck
  (params (RequestReload :type Boolean))
  (bind (_is_valid _weapon) (Weapon|GetActiveEquippedWeapon))
  ;[0 0 0] Check if ammo is not full, and if there is any reserve ammo left to draw from
  (if _is_valid
    (bind _output_get (LocalVariables|Setlocal_Weapon _weapon))
    (bind _output_get_2 (LocalVariables|Setlocal_CanReload (|GetCanReload _output_get)))
    (if _output_get_2
      (return (LocalVariables|Getlocal_CanReload))
      (else
        (if RequestReload
          (Variables|/Game/FPS_AnimBP_v2/Blueprints/Weapons/BP_WeaponBase.BP_WeaponBase_C|SetReloadRequested (LocalVariables|Getlocal_Weapon) (Variables|/Game/FPS_AnimBP_v2/Blueprints/Weapons/BP_WeaponBase.BP_WeaponBase_C|GetIsMidBurstFire (LocalVariables|Getlocal_Weapon))))
        (return (LocalVariables|Getlocal_CanReload))))
    (else
      (return false))))

(fn TryRecieveAmmo
  (params (AmmoDataAsset :type FPS%20PDA%20Ammo%20Data%20Base%20Object%20Reference) (Ammo%20Amount%20Override :type Integer))
  (bind (_is_valid _weapon) (Weapon|GetActiveEquippedWeapon))
  (bind _reserveammodata (Variables|LiveData|GetReserveAmmoData))
  (bind (_value _returnvalue) (Utilities|Map|Find _reserveammodata AmmoDataAsset))
  (Utilities|FlowControl|Sequence
    (:then_0
      (LocalVariables|Setlocal_AmmoToPickup (Variables|/Game/FPS_AnimBP_v2/Blueprints/DataAssets/Ammo/FPS_PDA_AmmoDataBase.FPS_PDA_AmmoDataBase_C|GetAmmoPerPickup AmmoDataAsset))
      (LocalVariables|Setlocal_MaxReserveAmmo (Variables|/Game/FPS_AnimBP_v2/Blueprints/DataAssets/Ammo/FPS_PDA_AmmoDataBase.FPS_PDA_AmmoDataBase_C|GetMaxReserveAmmo AmmoDataAsset))
      (Utilities|FlowControl|Sequence
        (:then_0
          ;[0 0 0] 1. Override the Ammo to Pickup if Ammo Amount Override != 0
          ; 2. If the Ammo Category is not already present in the inventory, current ammo before pickup defaults to 0. Otherwise, get the current ammo of the correct category. If the current ammo is already full, this ammo cannot be picked up.
          ; 3. Add the ammo to the ammo category's amount, or add it to the map if it did not already exist there
          (if (!= Ammo%20Amount%20Override 0)
            (LocalVariables|Setlocal_AmmoToPickup Ammo%20Amount%20Override)))
        (:then_1
          (if _returnvalue
            (bind _output_get (LocalVariables|Setlocal_CurrentAmmo _value))
            (if (not (< _output_get (LocalVariables|Getlocal_MaxReserveAmmo)))
              (return false))
            (else
              (LocalVariables|Setlocal_CurrentAmmo 0))))
        (:then_2
          (Utilities|Map|Add (Variables|LiveData|GetReserveAmmoData) AmmoDataAsset (Math|Integer|Clamp(Integer) (+ (LocalVariables|Getlocal_CurrentAmmo) (LocalVariables|Getlocal_AmmoToPickup)) 0 (LocalVariables|Getlocal_MaxReserveAmmo)))
          (if _is_valid
            (bind _current_reserve_ammo (Ammo|GetCurrentReserveAmmo))
            (Default|UpdateonGunAmmoCounter _weapon _current_reserve_ammo)))))
    (:then_1
      (return true))))

(fn GetAmmoCountsforActiveWeapon
  (bind (_is_valid _weapon) (Weapon|GetActiveEquippedWeapon))
  ;[0 0 0] Get all the ammo counts needed for the HUD
  (Utilities|FlowControl|Sequence
    (:then_0
      (if _is_valid
        (LocalVariables|Setlocal_MagazineSize (Default|GetMagazineSize _weapon))
        (LocalVariables|Setlocal_CurrentAmmo (.Current%20Ammo (Ammo|GetCurrentAmmo)))
        (bind (_weapon_is_valid _current_reserve_ammo _ammo_category) (Ammo|GetCurrentReserveAmmo))
        (LocalVariables|Setlocal_CurrentReserveAmmo _current_reserve_ammo)
        (LocalVariables|Setlocal_AmmoCategory _ammo_category)
        (else
          (return false 0 0 0))))
    (:then_1
      (return true (LocalVariables|Getlocal_CurrentAmmo) (LocalVariables|Getlocal_MagazineSize) (LocalVariables|Getlocal_CurrentReserveAmmo)))))

(fn GetCurrentReserveAmmo
  (bind (_is_valid _weapon) (Weapon|GetActiveEquippedWeapon))
  (bind _reserveammodata (Variables|LiveData|GetReserveAmmoData))
  (bind _ammotype (Default|GetAmmoType _weapon))
  (bind (_value _returnvalue) (Utilities|Map|Find _reserveammodata _ammotype))
  ;[0 0 0] Get the current reserve ammo and its category if the weapon is valid
  (if _is_valid
    (if _returnvalue
      (LocalVariables|Setlocal_ReserveAmmo _value)
      (else
        (LocalVariables|Setlocal_ReserveAmmo 0)))
    (return true (LocalVariables|Getlocal_ReserveAmmo) (Variables|/Game/FPS_AnimBP_v2/Blueprints/DataAssets/Ammo/FPS_PDA_AmmoDataBase.FPS_PDA_AmmoDataBase_C|GetAmmoCategory _ammotype) _ammotype)
    (else
      (return false 0 "NewEnumerator4" 0))))

(fn GetCurrentAmmo
  (bind (_is_valid _weapon) (Weapon|GetActiveEquippedWeapon))
  (if _is_valid
    (return true (Variables|/Game/FPS_AnimBP_v2/Blueprints/Weapons/BP_WeaponBase.BP_WeaponBase_C|GetCurrentAmmo _weapon))
    (else
      (return false 0))))

(fn SetReserveAmmoDefaults
  ;[0 0 0] Set some default starting values for reserve ammo counts
  (bind _keys (Utilities|Map|Keys (Variables|LiveData|GetReserveAmmoData)))
  (for _array_element _keys
    (Utilities|Map|Add (Variables|LiveData|GetReserveAmmoData) _array_element (Variables|/Game/FPS_AnimBP_v2/Blueprints/DataAssets/Ammo/FPS_PDA_AmmoDataBase.FPS_PDA_AmmoDataBase_C|GetDefaultReserveAmmo _array_element))))

(fn ReloadWeapon
  ;[0 0 0] Reload the weapon from the ammo inventory using the correct ammo category
  (bind (_weapon_is_valid _current_reserve_ammo _ammo_category _ammo_data_asset) (Ammo|GetCurrentReserveAmmo))
  (bind (_currentammo _magazinesize _reserveammo) (Default|AddCurrentAmmo (.Weapon (Weapon|GetActiveEquippedWeapon)) _current_reserve_ammo))
  (Utilities|Map|Add (Variables|LiveData|GetReserveAmmoData) _ammo_data_asset _reserveammo)
  (return _currentammo _magazinesize _reserveammo))

(fn OnPlayerDeath
  ;[0 0 0] Temporarily save the weapon inventory data so the weapon actors can be respawned with the player
  (Variables|LiveData|SetTempEquippedWeaponData (Weapon|GetWeaponInventoryData))
  (Weapon|DestroyWeaponActors))

(fn OnPlayerSpawned
  (params (OnLoadGame :type Boolean))
  (bind _activeequippedweaponindex (Variables|LiveData|GetActiveEquippedWeaponIndex))
  (bind _activeequippedweaponindex_2 (Variables|LiveData|GetActiveEquippedWeaponIndex))
  ;[0 0 0] When the player spawns, if a save game was loaded first, equip the current weapon. If not, restore the weapon inventory from the temp data and equip as needed
  (if OnLoadGame
    (Weapon|SetSwitchtoIndex _activeequippedweaponindex_2)
    (Weapon|EquipActiveWeapon _activeequippedweaponindex_2)
    (else
      (for (_array_element _array_index) (Variables|LiveData|GetTempEquippedWeaponData)
        (if (Utilities|Enum|NotEqual(Enum) (Variables|/Game/FPS_AnimBP_v2/Blueprints/DataAssets/Weapons/FPS_PDA_WeaponBase.FPS_PDA_WeaponBase_C|GetWeaponType (Utilities|Struct|BreakST_GunData _array_element)) "NewEnumerator0")
          (bind _spawned_weapon (Weapon|SpawnWeapon _array_element _array_index false))
          (Rendering|SetActorHiddenInGame _spawned_weapon true)
          (Attachments|EquipAllCurrentAttachmentsonWeapon _spawned_weapon)))
      (Utilities|IsWeaponValid _activeequippedweaponindex
        (:Is%20Valid
          (Weapon|SetSwitchtoIndex _activeequippedweaponindex)
          (if (not (Variables|LiveData|GetWeaponIsHolstered))
            (Weapon|EquipActiveWeapon _activeequippedweaponindex)))))))

(fn GetAttachmentsInventory
  (return (Variables|LiveData|GetAttachmentAssetsInventory)))

(fn OnChangeAttachment
  (params (Weapon%20Index :type Integer) (Attachment%20Slot :type E_AttachmentSlot%20Enum :default "NewEnumerator2") (Attachment%20Asset%20Data :type FPS%20PDA%20Attachment%20Data%20Base%20Object%20Reference))
  ;[0 0 0] Handle the equipping and unequipping of an attachment to the selected weapon if it is valid
  (bind _weapon (Utilities|GetWeaponatIndex Weapon%20Index)
    (:Is%20Valid
      (LocalVariables|Setlocal_Weapon _weapon)
      (Utilities|IsValid Attachment%20Asset%20Data
        (:Is%20Valid
          (bind _success (Attachments|EquipWeaponAttachment (LocalVariables|Getlocal_Weapon) Attachment%20Asset%20Data))
          (return _success))
        (:Is%20Not%20Valid
          (Attachments|UnequipAttachment Weapon%20Index Attachment%20Slot)
          (return true))))
    (:Is%20Not%20Valid
      (return false))))

(fn UnequipAttachment
  (params (Weapon%20Index :type Integer) (Attachment%20Slot :type E_AttachmentSlot%20Enum :default "NewEnumerator2"))
  (bind _weapon (Utilities|GetWeaponatIndex Weapon%20Index)
    (:Is%20Valid
      (Default|UnequipAttachment _weapon Attachment%20Slot))))

(fn InitializeInventory
  ;[0 0 0] Set the limit to the maximum number of weapons that can be held at a time
  (Utilities|Array|Resize (Variables|LiveData|GetEquippedWeapons) (Variables|Cusomisation|GetMaxEquippedWeapons))
  (Ammo|SetReserveAmmoDefaults))

(fn SetOwningController
  (params (Player%20Controller :type Player%20Controller%20Object%20Reference))
  (Variables|Default|SetOwningController Player%20Controller))

(fn GetReserveAmmobyCategory
  (params (Ammo%20Data%20Asset :type FPS%20PDA%20Ammo%20Data%20Base%20Object%20Reference%20%28by%20ref%29))
  (bind _reserveammodata (Variables|LiveData|GetReserveAmmoData))
  (bind (_value _returnvalue) (Utilities|Map|Find _reserveammodata Ammo%20Data%20Asset))
  ;[0 0 0] Get the reserve ammo of the selected ammo category
  (if _returnvalue
    (LocalVariables|Setlocal_ReserveAmmo _value)
    (else
      (LocalVariables|Setlocal_ReserveAmmo 0)))
  (return (LocalVariables|Getlocal_ReserveAmmo)))

(fn HolsterWeapon
  (bind (_is_valid _weapon) (Weapon|GetActiveEquippedWeapon))
  ;[0 0 0] Holster the current weapon and set the weapon to inactive
  (if _is_valid
    (Default|SetIsActiveWeapon _weapon false))
  (Variables|LiveData|SetWeaponIsHolstered true))

(fn UnholsterWeapon
  (bind _activeequippedweaponindex (Variables|LiveData|GetActiveEquippedWeaponIndex))
  ;[0 0 0] Re equip a holstered weapon
  (Utilities|IsWeaponValid _activeequippedweaponindex
    (:Is%20Valid
      (Weapon|EquipActiveWeapon _activeequippedweaponindex)
      (return true))
    (:Is%20Not%20Valid
      (bind _can_switch_weapon (Weapon|CycleWeapon true))
      (return _can_switch_weapon))))

(fn GetAmmoInventory
  (return (Variables|LiveData|GetReserveAmmoData)))

(fn GetAllInventories
  (return (Weapon|GetWeaponInventoryData) (Variables|LiveData|GetAttachmentAssetsInventory) (Variables|LiveData|GetReserveAmmoData) (Variables|LiveData|GetActiveEquippedWeaponIndex)))

(fn LoadInventoriesfromSave
  (params (AttachmentAssetsInventory :type Array%20of%20FPS%20PDA%20Attachment%20Data%20Base%20Object%20References) (ReserveAmmoData :type Map%20of%20FPS%20PDA%20Ammo%20Data%20Base%20Object%20References%20to%20Integers) (Inventory%20Data :type Array%20of%20ST%20Gun%20Data%20Structures) (ActiveEquippedWeaponIndex :type Integer))
  ;[0 0 0] Restore all inventories from a save file
  (Variables|LiveData|SetAttachmentAssetsInventory AttachmentAssetsInventory)
  (Variables|LiveData|SetReserveAmmoData ReserveAmmoData)
  (Weapon|RestoreFullInventory Inventory%20Data ActiveEquippedWeaponIndex))

(fn EquipAllCurrentAttachmentsonWeapon
  (params (Weapon :type BP%20Weapon%20Base%20Object%20Reference))
  (bind _weaponattachments (Variables|/Game/FPS_AnimBP_v2/Blueprints/Weapons/BP_WeaponBase.BP_WeaponBase_C|GetWeaponAttachments Weapon))
  (bind (_sights _muzzle _magazine _underbarrel _stock) (Utilities|Struct|BreakST_WeaponAttachments _weaponattachments))
  ;[0 0 0] Equip all the attachments specified in the Attachments list. For magazine, if no attachment is specified, fall back to the default magazine for that weapon, as one magazine must be equipped
  (Attachments|EquipWeaponAttachment Weapon _sights)
  (Attachments|EquipWeaponAttachment Weapon _muzzle)
  (Attachments|EquipWeaponAttachment Weapon _magazine)
  (Attachments|EquipWeaponAttachment Weapon _underbarrel)
  (Attachments|EquipWeaponAttachment Weapon _stock))