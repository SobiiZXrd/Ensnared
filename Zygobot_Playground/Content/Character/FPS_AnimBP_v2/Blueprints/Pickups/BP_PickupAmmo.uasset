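; Ammo pickup Blueprint that the player collects by walking over it rather than interacting manually.
; Sphere overlap by the player sends the ammo data asset and optional spawner-set amount override through RecieveAmmoMessage, then fires OnPickup and destroys the pickup only if accepted.
; On BeginPlay, the ammo category sets the mesh material and front/back labels, or prints an error if it is None.
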(event OnComponentBeginOverlap(Sphere)
  (params (OverlappedComponent :type Primitive%20Component%20Object%20Reference) (OtherActor :type Actor%20Object%20Reference) (OtherComp :type Primitive%20Component%20Object%20Reference) (OtherBodyIndex :type Integer) (bFromSweep :type Boolean) (SweepResult :type Hit%20Result%20Structure%20%28by%20ref%29))
  ;[0 0 0] This pickup is automatically interacted with by overlapping it rather than by manual interaction
  (if (== (Game|GetPlayerCharacter 0) OtherActor)
    (CallFunction|OnInteract OtherActor)))

(event EventBeginPlay
  ;[0 0 0] Check if the ammo has valid settings when spawned
  (CallFunction|CheckifAmmoIsValid))

(event EventInteract
  (params (InteractingActor :type Actor%20Object%20Reference))
  ;[0 0 0] This pickup is automatically interacted with by overlapping it rather than by manual interaction
)

(fn ConstructionScript
  (|CallParentFunction)
  (Components|DestroyComponent (Variables|Default|GetSkeletalMesh))
  (Transformation|AttachComponentToComponent (Variables|Default|GetSphere) (Variables|Default|GetStaticMesh) "root" "KeepRelative" "KeepRelative" "KeepRelative" true))

(fn OnInteract
  (params (InteractingActor :type Actor%20Object%20Reference))
  ;[0 0 0] Attempt to send the ammo to the player. If the player could not pick this up, leave it alone, otherwise destroy this pickup.
  ; Override the default ammo picked up if AmmoAmountOverride != 0, which is determined by whatever spawned this pickup.
  (bind _success (Class|BPCharacterInterface|RecieveAmmo(Message) InteractingActor (Variables|Default|GetAmmoDataAsset) (Variables|Default|GetAmmoAmountOverride)))
  (if _success
    (Default|CallOnPickup)
    (Actor|DestroyActor)))

(fn CheckifAmmoIsValid
  ;[0 0 0] If Ammo Category is none, print an error and destroy this pickup. Otherwise, set the colour and label
  (if (Utilities|Enum|Equal(Enum) (Variables|/Game/FPS_AnimBP_v2/Blueprints/DataAssets/Ammo/FPS_PDA_AmmoDataBase.FPS_PDA_AmmoDataBase_C|GetAmmoCategory (Variables|Default|GetAmmoDataAsset)) "NewEnumerator4")
    (|PrintErrorInvalidAmmoCategory)
    (else
      (CallFunction|SetPickupFX))))

(fn SetPickupFX
  (Rendering|Material|SetMaterial (Variables|Default|GetStaticMesh) 0 (Utilities|Select :Index (Variables|/Game/FPS_AnimBP_v2/Blueprints/DataAssets/Ammo/FPS_PDA_AmmoDataBase.FPS_PDA_AmmoDataBase_C|GetAmmoCategory (Variables|Default|GetAmmoDataAsset)) :NewEnumerator4 "/Game/FPS_AnimBP_v2/Demo/DemoRoom/Materials/M_DemoRoomTiles_Inst_Color5_Inst.M_DemoRoomTiles_Inst_Color5_Inst" :NewEnumerator0 "/Game/FPS_AnimBP_v2/Demo/DemoRoom/Materials/M_DemoRoomTiles_Inst_Color5_Inst.M_DemoRoomTiles_Inst_Color5_Inst" :NewEnumerator1 "/Game/FPS_AnimBP_v2/Demo/DemoRoom/Materials/M_DemoRoomTiles_Inst_Color6.M_DemoRoomTiles_Inst_Color6" :NewEnumerator2 "/Game/FPS_AnimBP_v2/Demo/DemoRoom/Materials/M_DemoRoomTiles_Inst_Color2.M_DemoRoomTiles_Inst_Color2" :NewEnumerator3 "/Game/FPS_AnimBP_v2/Demo/DemoRoom/Materials/M_DemoRoomTiles_Inst_Color3.M_DemoRoomTiles_Inst_Color3"))
  (Rendering|Components|TextRender|SetText (Variables|Default|GetAmmoLabelFront) (Utilities|Text|ToText(String) (Utilities|String|EnumtoString (Variables|/Game/FPS_AnimBP_v2/Blueprints/DataAssets/Ammo/FPS_PDA_AmmoDataBase.FPS_PDA_AmmoDataBase_C|GetAmmoCategory (Variables|Default|GetAmmoDataAsset))))))