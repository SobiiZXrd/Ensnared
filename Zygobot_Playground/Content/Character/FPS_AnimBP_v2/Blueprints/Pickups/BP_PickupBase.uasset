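; BP_PickupBase is the parent Blueprint for interactable pickups, leaving SetPickupMesh and OnInteract empty for subclasses to override.
; InitiliazePickup runs at construction and BeginPlay to set the mesh, configure the optional point light, and toggle physics and gravity on valid skeletal or static meshes.
; Interact forwards to OnInteract, while GetButtonPromptInfo returns a device-specific key with the prompt hidden by default.
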(event EventBeginPlay
  ;[0 0 0] Initialise the pickup on creation
  (CallFunction|InitiliazePickup))

(event EventInteract
  (params (InteractingActor :type Actor%20Object%20Reference))
  ;[0 0 0] Manual interaction through a button press
  (CallFunction|OnInteract InteractingActor))

(fn ConstructionScript
  (CallFunction|InitiliazePickup))

(fn SetPickupMesh
  ;[0 0 0] Override for subclasses
)

(fn OnInteract
  (params (InteractingActor :type Actor%20Object%20Reference))
  ;[0 0 0] Override for subclasses
)

(fn InitiliazePickup
  (bind _pointlight (Variables|Default|GetPointLight))
  ;[0 0 0] Set the meshes, VFX, and physics behaviour
  (CallFunction|SetPickupMesh)
  (Rendering|Components|Light|SetIntensity _pointlight (select (Variables|Default|GetEnableLight) (Variables|Default|GetLightIntensity) 0.0))
  (Rendering|Components|Light|SetLightColor _pointlight (Variables|Default|GetLightColour) true)
  (CallFunction|SetPhysics))

(fn SetPhysics
  (bind _enablephysics (Variables|Default|GetEnablePhysics))
  (bind _enablephysics_2 (Variables|Default|GetEnablePhysics))
  ;[0 0 0] Turn the on or off on the relavent mesh(es)
  (Utilities|FlowControl|Sequence
    (:then_0
      (bind _skeletalmesh (Variables|Default|GetSkeletalMesh)
        (:then
          (Physics|SetSimulatePhysics _skeletalmesh _enablephysics_2)
          (Physics|SetEnableGravity _skeletalmesh _enablephysics_2))
        (:else)))
    (:then_1
      (bind _staticmesh (Variables|Default|GetStaticMesh)
        (:then
          (Physics|SetSimulatePhysics _staticmesh _enablephysics)
          (Physics|SetEnableGravity _staticmesh _enablephysics))
        (:else)))))

(fn GetButtonPromptInfo
  (return false (Utilities|Select :Index (CallFunction|GetCurrentInputDevice) :NewEnumerator0 "F" :NewEnumerator1 "Right Face Button") "Interact"))