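; World pickup for a weapon attachment, configured by an attachment data asset and extending a parent pickup class.
; It displays the asset's skeletal mesh, falling back to its static mesh, attaches the collision sphere to that component, and reports invalid data as errors.
; On interact it sends the data asset to the interacting actor and destroys itself only on success.
; Its prompt shows the attachment name with a device-specific key.
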(event EventBeginPlay)

(event Collision|EventActorBeginOverlap
  (params (OtherActor :type Actor%20Object%20Reference)))

(event EventTick
  (params (DeltaSeconds :type Float%20%28single-precision%29)))

(fn ConstructionScript
  (|CallParentFunction))

(fn InitiliazePickup
  ;[0 0 0] Destroy the unused Static Mesh component, and attach the collision detection sphere to the skeletal mesh
  (|CallParentFunction)
  (Transformation|AttachComponentToComponent (Variables|Default|GetSphere) (Variables|Default|GetSkeletalMesh) "None" "KeepRelative" "KeepRelative" "KeepRelative" false))

(fn SetPickupMesh
  (bind _skeletalmesh (Variables|Default|GetSkeletalMesh))
  (bind _staticmesh (Variables|Default|GetStaticMesh))
  ;[0 0 0] Set the mesh used by the pickup in the world
  (bind _attachmentdataasset (Variables|AttachmentPickupSettings|GetAttachmentDataAsset)
    (:then
      (Utilities|IsValid (.SkeletalMesh (Default|GetAttachmentBaseData _attachmentdataasset))
        (:Is%20Valid
          (Class|SkinnedMeshComponent|SetSkeletalMesh _skeletalmesh (.SkeletalMesh (Default|GetAttachmentBaseData _attachmentdataasset)) true)
          (Transformation|AttachComponentToComponent (Variables|Default|GetSphere) _skeletalmesh "None" "KeepRelative" "KeepRelative" "KeepRelative" true))
        (:Is%20Not%20Valid
          (Utilities|IsValid (.MainStaticMesh (Default|GetAttachmentBaseData _attachmentdataasset))
            (:Is%20Valid
              (Components|StaticMesh|SetStaticMesh _staticmesh (.MainStaticMesh (Default|GetAttachmentBaseData _attachmentdataasset)))
              (Transformation|AttachComponentToComponent (Variables|Default|GetSphere) _staticmesh "None" "KeepRelative" "KeepRelative" "KeepRelative" true))
            (:Is%20Not%20Valid
              (|PrintErrorInvalidAttachmentMesh))))))
    (:else
      (|PrintErrorInvalidAttachmentDataAsset))))

(fn OnInteract
  (params (InteractingActor :type Actor%20Object%20Reference))
  ;[0 0 0] When the pickup is interacted with, send the attachment data to the interacting player. If this succeeds, destroy this pickup
  (bind _success (Class|BPCharacterInterface|RecieveWeaponAttachment(Message) InteractingActor (Variables|AttachmentPickupSettings|GetAttachmentDataAsset)))
  (if _success
    (Actor|DestroyActor)))

(fn GetButtonPromptInfo
  ;[0 0 0] Get the information to be displayed on the Interact Prompt
  (return true (Utilities|Select :Index (CallFunction|GetCurrentInputDevice) :NewEnumerator0 "F" :NewEnumerator1 "Right Face Button") (Utilities|Text|FormatText "Pick Up {Name}" (Variables|/Game/FPS_AnimBP_v2/Blueprints/DataAssets/FPS_PDA_ItemDataBase.FPS_PDA_ItemDataBase_C|GetDisplay%20Name (Variables|AttachmentPickupSettings|GetAttachmentDataAsset)))))