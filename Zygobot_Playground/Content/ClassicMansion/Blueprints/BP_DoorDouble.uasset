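; Double door for the Classic Mansion that swings open when an actor overlaps it and closes when overlap ends, or opens at BeginPlay if Open is set.
; The construction script adds left and right skeletal meshes and picks their animations from four styles by DoorType.
; Each leaf plays its animation while a timeline drives its yaw, reversed to close, with added audio.
; An Opening flag blocks re-triggering and delays closing mid-swing.
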(event EventBeginPlay
  (bind _doorl (Variables|Default|GetDoorL))
  (bind _doorr (Variables|Default|GetDoorR))
  (if (Variables|Default|GetOpen)
    (if (not (Variables|Default|GetOpening))
      (Variables|Default|SetOpening true)
      (Utilities|FlowControl|Sequence
        (:then_0
          (AddComponent|AddAudioComponent false)
          (Components|Animation|PlayAnimation _doorr (Variables|Default|GetAnimR) false)
          (bind _newtrack_0 (Timeline|Timeline_0 Play)
            (:Update
              (Transformation|SetRelativeRotation _doorr (Math|Rotator|MakeRotator 0.0 0.0 _newtrack_0) false false))
            (:Finished
              (Variables|Default|SetOpening false))))
        (:then_1
          (Components|Animation|PlayAnimation _doorl (Variables|Default|GetAnimL) false)
          (bind _newtrack_0_2 (Timeline|Timeline_1 Play)
            (:Update
              (Transformation|SetRelativeRotation _doorl (Math|Rotator|MakeRotator 0.0 0.0 _newtrack_0_2) false false))))))))

(event Collision|EventActorBeginOverlap
  (params (OtherActor :type Actor%20Object%20Reference))
  (bind _doorl (Variables|Default|GetDoorL))
  (bind _doorr (Variables|Default|GetDoorR))
  (if (not (Variables|Default|GetOpen))
    (if (not (Variables|Default|GetOpening))
      (Variables|Default|SetOpening true)
      (Utilities|FlowControl|Sequence
        (:then_0
          (AddComponent|AddAudioComponent false)
          (Components|Animation|PlayAnimation _doorr (Variables|Default|GetAnimR) false)
          (bind _newtrack_0 (Timeline|Timeline_0 Play)
            (:Update
              (Transformation|SetRelativeRotation _doorr (Math|Rotator|MakeRotator 0.0 0.0 _newtrack_0) false false))
            (:Finished
              (Variables|Default|SetOpening false))))
        (:then_1
          (Components|Animation|PlayAnimation _doorl (Variables|Default|GetAnimL) false)
          (bind _newtrack_0_2 (Timeline|Timeline_1 Play)
            (:Update
              (Transformation|SetRelativeRotation _doorl (Math|Rotator|MakeRotator 0.0 0.0 _newtrack_0_2) false false))))))))

(event Collision|EventActorEndOverlap
  (params (OtherActor :type Actor%20Object%20Reference))
  (bind _doorl (Variables|Default|GetDoorL))
  (bind _doorr (Variables|Default|GetDoorR))
  (if (not (Variables|Default|GetOpen))
    (if (Variables|Default|GetOpening)
      (Utilities|FlowControl|RetriggerableDelay 1.0))
    (Utilities|FlowControl|Sequence
      (:then_0
        (AddComponent|AddAudioComponent false)
        (Components|Animation|PlayAnimation _doorr (Variables|Default|GetAnimR) false)
        (bind _newtrack_0 (Timeline|Timeline_0 Reverse)
          (:Update
            (Transformation|SetRelativeRotation _doorr (Math|Rotator|MakeRotator 0.0 0.0 _newtrack_0) false false))
          (:Finished
            (Variables|Default|SetOpening false))))
      (:then_1
        (Components|Animation|PlayAnimation _doorl (Variables|Default|GetAnimL) false)
        (bind _newtrack_0_2 (Timeline|Timeline_1 Reverse)
          (:Update
            (Transformation|SetRelativeRotation _doorl (Math|Rotator|MakeRotator 0.0 0.0 _newtrack_0_2) false false)))))))

(event EventTick
  (params (DeltaSeconds :type Float%20%28single-precision%29)))

(fn ConstructionScript
  (bind _doortype (Variables|Default|GetDoorType))
  (bind _returnvalue (Math|Conversions|ToFloat(Integer) _doortype))
  (if (Math|Float|InRange(Float) _returnvalue 0.0 1.0 false)
    (bind _returnvalue_2 (AddComponent|AddSkeletalMeshComponent false (Math|Transform|MakeTransform "-78.000000,-1.750000, 0" "0, 0, 0" "1,1,1")))
    (Variables|Default|SetDoorL _returnvalue_2)
    (Variables|Default|SetAnimL "/Game/ClassicMansion/Meshes/SK_DoorA_L_Anim.SK_DoorA_L_Anim")
    (bind _returnvalue_3 (AddComponent|AddSkeletalMeshComponent false (Math|Transform|MakeTransform "78.000000,-1.750000, 0" "0, 0, 0" "1,1,1")))
    (Variables|Default|SetDoorR _returnvalue_3)
    (Variables|Default|SetAnimR "/Game/ClassicMansion/Meshes/SK_DoorA_R_Anim.SK_DoorA_R_Anim")
    (elif (Math|Float|InRange(Float) _returnvalue 1.0 2.0 false)
      (bind _returnvalue_4 (AddComponent|AddSkeletalMeshComponent false (Math|Transform|MakeTransform "-78.000000,-1.750000, 0" "0, 0, 0" "1,1,1")))
      (Variables|Default|SetDoorL _returnvalue_4)
      (Variables|Default|SetAnimL "/Game/ClassicMansion/Meshes/SK_DoorB_L_Anim.SK_DoorB_L_Anim")
      (bind _returnvalue_5 (AddComponent|AddSkeletalMeshComponent false (Math|Transform|MakeTransform "78.000000,-1.750000, 0" "0, 0, 0" "1,1,1")))
      (Variables|Default|SetDoorR _returnvalue_5)
      (Variables|Default|SetAnimR "/Game/ClassicMansion/Meshes/SK_DoorB_R_Anim.SK_DoorB_R_Anim")
      (elif (Math|Float|InRange(Float) _returnvalue 2.0 3.0 false)
        (bind _returnvalue_6 (AddComponent|AddSkeletalMeshComponent false (Math|Transform|MakeTransform "-78.000000,-1.750000, 0" "0, 0, 0" "1,1,1")))
        (Variables|Default|SetDoorL _returnvalue_6)
        (Variables|Default|SetAnimL "/Game/ClassicMansion/Meshes/SK_DoorC_L_Anim.SK_DoorC_L_Anim")
        (bind _returnvalue_7 (AddComponent|AddSkeletalMeshComponent false (Math|Transform|MakeTransform "78.000000,-1.750000, 0" "0, 0, 0" "1,1,1")))
        (Variables|Default|SetDoorR _returnvalue_7)
        (Variables|Default|SetAnimR "/Game/ClassicMansion/Meshes/SK_DoorC_R_Anim.SK_DoorC_R_Anim")
        (elif (Math|Float|InRange(Float) _returnvalue 3.0 4.0 false)
          (bind _returnvalue_8 (AddComponent|AddSkeletalMeshComponent false (Math|Transform|MakeTransform "-78.000000,-1.750000, 0" "0, 0, 0" "1,1,1")))
          (Variables|Default|SetDoorL _returnvalue_8)
          (Variables|Default|SetAnimL "/Game/ClassicMansion/Meshes/SK_DoorD_L_Anim.SK_DoorD_L_Anim")
          (bind _returnvalue_9 (AddComponent|AddSkeletalMeshComponent false (Math|Transform|MakeTransform "78.000000,-1.750000, 0" "0, 0, 0" "1,1,1")))
          (Variables|Default|SetDoorR _returnvalue_9)
          (Variables|Default|SetAnimR "/Game/ClassicMansion/Meshes/SK_DoorD_R_Anim.SK_DoorD_R_Anim"))))))