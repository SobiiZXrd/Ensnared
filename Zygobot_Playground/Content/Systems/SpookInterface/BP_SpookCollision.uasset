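; BP_SpookCollision is a trigger actor that causes spooky events when a Player-tagged actor overlaps its SpookCatalyst component.
; Overlap fires Activate, which loops through SpookSounds at the actor's location with a Delay per sound, and sends activate messages to every SpookElements entry.
; Ending the overlap sends those elements deactivate messages, but sounds are not stopped: the actor's Deactivate event is empty and the stop logic is unwired.
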(event OnComponentBeginOverlap(SpookCatalyst)
  (params (OverlappedComponent :type Primitive%20Component%20Object%20Reference) (OtherActor :type Actor%20Object%20Reference) (OtherComp :type Primitive%20Component%20Object%20Reference) (OtherBodyIndex :type Integer) (bFromSweep :type Boolean) (SweepResult :type Hit%20Result%20Structure%20%28by%20ref%29))
  ;[0 0 0] Causing Spooky events
  (if (Actor|ActorHasTag OtherActor "Player")
    (Utilities|FlowControl|Sequence
      (:then_0
        (CallFunction|Activate))
      (:then_1
        (for _array_element (Variables|SpookComponents|GetSpookElements)
          (Class|BPISpook|Activate(Message) _array_element))))))

(event OnComponentEndOverlap(SpookCatalyst)
  (params (OverlappedComponent :type Primitive%20Component%20Object%20Reference) (OtherActor :type Actor%20Object%20Reference) (OtherComp :type Primitive%20Component%20Object%20Reference) (OtherBodyIndex :type Integer))
  ;[0 0 0] Causing Spooky events
  (if (Actor|ActorHasTag OtherActor "Player")
    (for _array_element (Variables|SpookComponents|GetSpookElements)
      (Class|BPISpook|Deactivate(Message) _array_element))))

(event EventBeginPlay)

(event Collision|EventActorBeginOverlap
  (params (OtherActor :type Actor%20Object%20Reference)))

(event EventTick
  (params (DeltaSeconds :type Float%20%28single-precision%29)))

(event EventActivate
  ;[0 0 0] Causing Spooky events
  (for _array_element (Variables|SpookComponents|GetSpookSounds)
    (Audio|PlaySoundatLocation _array_element (Transformation|GetActorLocation self) "0, 0, 0" 1.0 1.0 0.0 "/Game/Systems/Sound/Attenuarion/Spook/FarSpook_SA.FarSpook_SA" 0 0 0)
    (Utilities|FlowControl|Delay (Variables|/Script/Engine.SoundBase|GetDuration _array_element)))
  (CallFunction|Deactivate))

(event EventDeactivate)

(fn ConstructionScript)