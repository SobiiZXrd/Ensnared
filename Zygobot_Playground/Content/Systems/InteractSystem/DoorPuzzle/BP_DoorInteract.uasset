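; BP_DoorInteract is the interactable escape door in the door puzzle system, opened by pressing E.
; BeginPlay clears its stored struct position and judgement flag while keeping its configured puzzle shape.
; On Interact it passes all three values to GetDoorPuzzleRefs, stores the returned judgement, then destroys itself without checking that result.
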(event EventBeginPlay
  ;[0.1006 0 1] BEGIN PLAY
  (Variables|Shape|SetCurrent_PuzzleShape (Variables|Shape|GetCurrent_PuzzleShape))
  (Variables|Shape|SetCurrent_StructPos "")
  (Variables|Shape|SetbCurrent_Judgement false))

(event Collision|EventActorBeginOverlap
  (params (OtherActor :type Actor%20Object%20Reference)))

(event EventTick
  (params (DeltaSeconds :type Float%20%28single-precision%29)))

(event EventInteract
  ;[1 0.09896 0.09896] Press "E" to interact to open the escape door.
  (Variables|Shape|SetbCurrent_Judgement (CallFunction|GetDoorPuzzleRefs (Variables|Shape|GetCurrent_PuzzleShape) (Variables|Shape|GetCurrent_StructPos) (Variables|Shape|GetbCurrent_Judgement)))
  (Actor|DestroyActor self))

(fn ConstructionScript)