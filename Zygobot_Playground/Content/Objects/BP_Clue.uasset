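; BP_Clue is an interactable, collectible narrative clue.
; It creates its clue widget on BeginPlay; Interact plays a paper crumple, registers the clue with the game mode, shows the widget, updates the player HUD and destroys the actor.
; Tick sets the widget image from the game mode's clue count, though overlapping comparisons leave the cone image unreachable.
; A separate SetClueDisplay function sets the paper texture directly.
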(event EventBeginPlay
  (bind _returnvalue (UserInterface|CreateWidget "/Game/Systems/UI_HUD/W_NarrativeClue_UI.W_NarrativeClue_UI_C"))
  (Variables|Default|SetW_NarrativeClue_Ref _returnvalue))

(event EventInteract
  (bind (_numberofclues _ensnaredgamemode) (CallFunction|GetGameModeVars))
  ;[0.6427 0.1858 1] INTERACT Event
  (Variables|Default|GetW_NarrativeClue_Ref
    (:then
      (Audio|PlaySound2D "/Game/Systems/Sound/WAV_Dump/turchinoa__paper-crumple.turchinoa__paper-crumple" 1.0 1.0 0.0 0 0)
      (Default|EventAddClue _ensnaredgamemode _numberofclues)
      (UserInterface|Viewport|AddtoViewport (Variables|Default|GetW_NarrativeClue_Ref) 0))
    (:else
      (bind _returnvalue (UserInterface|CreateWidget "/Game/Systems/UI_HUD/W_NarrativeClue_UI.W_NarrativeClue_UI_C"))
      (Variables|Default|SetW_NarrativeClue_Ref _returnvalue)))
  (Default|EventUpdateHUD (.PlayerChar_Ref (CallFunction|GetPlayerCharacterP)) (Variables|/Game/Systems/BPGM_Ensnared.BPGM_Ensnared_C|GetCurrentClues _ensnaredgamemode))
  (Actor|DestroyActor))

(event EventTick
  (params (DeltaSeconds :type Float%20%28single-precision%29))
  (bind _ensnaredgamemode (CallFunction|GetGameModeVars))
  (bind _currentclues (Variables|/Game/Systems/BPGM_Ensnared.BPGM_Ensnared_C|GetCurrentClues _ensnaredgamemode))
  ;[1 0 0] PER FRAME EVENTS
  ;[0.2812 0.27 0.06104] Changing UI Clue image depending on how many clues are currently held
  (if (>= _currentclues 1)
    (Default|UpdateClueImage (Variables|Default|GetW_NarrativeClue_Ref) "/Game/Systems/InteractSystem/DoorPuzzle/PuzzleSphereClue.PuzzleSphereClue")
    (elif (<= _currentclues 1)
      (Default|UpdateClueImage (Variables|Default|GetW_NarrativeClue_Ref) "/Game/Systems/InteractSystem/DoorPuzzle/PuzzleCubeClue.PuzzleCubeClue")
      (elif (>= _currentclues 2)
        (Default|UpdateClueImage (Variables|Default|GetW_NarrativeClue_Ref) "/Game/Systems/InteractSystem/DoorPuzzle/PuzzleConeClue.PuzzleConeClue")))))

(fn ConstructionScript)

(fn SetClueDisplay
  (params (CurrentClue_Ref :type Texture%202D%20Object%20Reference))
  ;[0.1823 0 0] Setting what clue to display
  (Appearance|SetBrushfromTexture (Variables|/Game/Systems/UI_HUD/W_NarrativeClue_UI.W_NarrativeClue_UI_C|GetPaperClue (Variables|Default|GetW_NarrativeClue_Ref)) CurrentClue_Ref false))