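; Escape door puzzle actor that displays the cone, sphere or cube pieces the player carries and can slide open.
; Interact reveals the first held shape in cone, sphere, cube priority and sets its placed flag.
; A separately triggered open event plays a sound and eases the door along world X by timeline.
; When the slide finishes, it clears the player's shape flags and marks the door open.
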(event Custom|Enter_OpenEscapeDoor
  (bind _playerchar_ref (CallFunction|GetPlayerCharacterP))
  ;[0.05208 0.05208 0.05208] Event Open Escape Door
  (if (not (Variables|OpenDoorComponents|GetbIsOpen?))
    (Audio|PlaySound2D "/Game/Systems/Sound/WAV_Dump/ertfelda__hidden-wall-opening.ertfelda__hidden-wall-opening" 1.0 1.0 0.0 0 0 false)
    (Variables|Default|SetOpen_EscapeDoor_Vector (Transformation|GetWorldLocation (Variables|Debug|GetStaticMeshComponent self)))
    (bind _tltrack_escaperoute1 (Timeline|TL_OpenEscapeDoor PlayFromStart)
      (:Update
        (Transformation|SetWorldLocation (Variables|Debug|GetStaticMeshComponent self) (Math|Interpolation|Ease "EaseInOut" _tltrack_escaperoute1 (Variables|Default|GetOpen_EscapeDoor_Vector) (Math|Vector|MakeVector (+ (.x (Variables|Default|GetOpen_EscapeDoor_Vector)) 5.5e+02) (.y (Variables|Default|GetOpen_EscapeDoor_Vector)) (.z (Variables|Default|GetOpen_EscapeDoor_Vector))) 0.15) false false))
      (:Finished
        (Variables|/Game/Character/Player/BP_PlayerZ.BP_PlayerZ_C|SetbHasCone _playerchar_ref false)
        (Variables|/Game/Character/Player/BP_PlayerZ.BP_PlayerZ_C|SetbHasCube _playerchar_ref false)
        (Variables|/Game/Character/Player/BP_PlayerZ.BP_PlayerZ_C|SetbHasSphere _playerchar_ref false)
        (Variables|OpenDoorComponents|SetbIsOpen? true)))))

(event EventBeginPlay
  ;[0.09423 0.1002 1] BEGIN PLAY
  (Rendering|SetVisibility (Variables|Default|GetPuzzleConeAppear) false false)
  (Variables|OpenDoorComponents|SetbIsOpen? false))

(event EventInteract
  (bind _playerchar_ref (CallFunction|GetPlayerCharacterP))
  ;[1 0 0] When looking at the particular shape on the escape door the door will show the placed shape in to its proper hole
  (if (Variables|/Game/Character/Player/BP_PlayerZ.BP_PlayerZ_C|GetbHasCone _playerchar_ref)
    (Rendering|SetVisibility (Variables|Default|GetPuzzleConeAppear) true false)
    (Variables|OpenDoorcomponents|SetbSetCone? true)
    (elif (Variables|/Game/Character/Player/BP_PlayerZ.BP_PlayerZ_C|GetbHasSphere _playerchar_ref)
      (Rendering|SetVisibility (Variables|Default|GetPuzzleSphereAppear) true false)
      (Variables|OpenDoorComponents|SetbSetSphere? true)
      (elif (Variables|/Game/Character/Player/BP_PlayerZ.BP_PlayerZ_C|GetbHasCube _playerchar_ref)
        (Rendering|SetVisibility (Variables|Default|GetPuzzleCubeAppear) true false)
        (Variables|OpenDoorComponents|SetbSetCube? true)))))

(fn ConstructionScript)