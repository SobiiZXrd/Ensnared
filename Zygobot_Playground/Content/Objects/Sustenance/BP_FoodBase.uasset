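; BP_FoodBase is a food actor, apparently a base class, that heals the player on interaction and is then consumed.
; It caches the player character on BeginPlay.
; On Interact, FSetHealAmount rolls a random value between an offset HealAmount and MaxHealAmount, which feeds the player's FHealPlayer.
; After a short delay, it plays a 2D eating sound and destroys itself.
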(event EventBeginPlay
  ;[0 0.0107 0.1615] BEGIN Play
  (Variables|Default|SetPlayer%20Char%20Ref (.PlayerChar_Ref (CallFunction|GetPlayerCharacterP))))

(event EventInteract
  ;[0.07812 0.05912 0] Upon player interaction: set a ranged random amount for healing amount, then heal the player.
  (CallFunction|FSetHealAmount (Variables|Default|GetHeal%20Amount))
  (Default|FHealPlayer (Variables|Default|GetPlayer%20Char%20Ref) (Variables|Default|GetHeal%20Amount))
  (Utilities|FlowControl|Delay 0.2)
  (Audio|PlaySound2D "/Game/Systems/Sound/Interaction/eating_Cue.eating_Cue" 1.0 1.0 0.0 0 0 false)
  (Actor|DestroyActor))

(fn ConstructionScript)

(fn FSetHealAmount
  (params (HealAmount :type Float%20%28double-precision%29))
  (Variables|Default|SetHeal%20Amount (Math|Random|RandomFloatinRange (+ HealAmount 5.0) (Variables|Default|GetMax_HealAmount))))