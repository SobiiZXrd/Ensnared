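; Door actor that animates a supplied rotator component between open and closed rotations.
; BeginPlay caches the root's world location and the actor's scale.
; Separate open and close events take the component and start and end rotations from the caller, then drive eased world rotation through their own timelines.
; Each timeline updates IsOpen when it finishes; the file contains no trigger or input logic.
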(event Custom|Enter_CloseDoor
  (params (Door_RotatorRef :type Static%20Mesh%20Component%20Object%20Reference) (Door_CurRotation :type Rotator) (Door_NewRotation :type Rotator))
  ;[0 0 0] Open and close Door events
  (bind _newtrack_0 (Timeline|DoorClose_TL Play)
    (:Update
      (Transformation|SetWorldRotation Door_RotatorRef (Math|Interpolation|Ease "EaseOut" _newtrack_0 Door_CurRotation Door_NewRotation false) false false))
    (:Finished
      (Variables|OpenCloseEvents|SetbIsOpen? false))))

(event Custom|Enter_OpenDoor
  (params (Door_CurRotation :type Rotator) (Door_NewRotation :type Rotator) (Door_RotatorRef :type Static%20Mesh%20Component%20Object%20Reference))
  ;[0 0 0] Open and close Door events
  (bind _opendoor_fltrack (Timeline|TL_OpenDoor Play)
    (:Update
      (Transformation|SetWorldRotation Door_RotatorRef (Math|Interpolation|Ease "EaseInOut" _opendoor_fltrack Door_CurRotation Door_NewRotation true) false false))
    (:Finished
      (Variables|OpenCloseEvents|SetbIsOpen? true))))

(event EventBeginPlay
  (bind _self self)
  (Variables|Components|SetDoor_OGLocation (Transformation|GetWorldLocation (Variables|Default|GetDefaultSceneRoot _self)))
  (Variables|Components|SetDoor_OG3DScale (Transformation|GetActorScale3D _self)))

(event EventTick
  (params (DeltaSeconds :type Float%20%28single-precision%29)))

(fn ConstructionScript)