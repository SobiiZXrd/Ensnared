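; BP_DungeonDoor is an interactable dungeon door that swings open or closed with a matching sound.
; BeginPlay stores the Rotator component's world rotation as the original orientation.
; Interact branches on IsOpen, offsetting yaw by the open angle through ClampAngle, from the stored rotation to open or the current one to close.
; The target rotation feeds EnterOpenDoor or EnterCloseDoor, whose bodies are not defined here.
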(event EventBeginPlay
  ;[0 0.001442 0.03125] BEGIN PLAY EVENTS
  (|CallParentFunction)
  (Variables|DoorOpen&CloseEvents|SetDungeonDoor_OGRotation (Transformation|GetWorldRotation (Variables|DoorOpen&CloseEvents|GetRotator))))

(event EventTick
  (params (DeltaSeconds :type Float%20%28single-precision%29))
  (|CallParentFunction DeltaSeconds) ; This node is disabled and will not be called.\nDrag off pins to build functionality.
)

(event EventInteract
  (bind _dungeondoor_ogrotation (Variables|DoorOpen&CloseEvents|GetDungeonDoor_OGRotation))
  (bind _opendoor_rotangle (Variables|Door_Open&Close_Events|GetOpenDoor_RotAngle))
  (bind _opendoor_rotangle_2 (Variables|Door_Open&Close_Events|GetOpenDoor_RotAngle))
  ;[0 0 0] Open Door upon player interaction
  (if (not (Variables|Default|GetbIsOpen?))
    (Audio|PlaySoundatLocation "/Game/ClassicMansion/Audio/Cues/SC_DoorOpen.SC_DoorOpen" (Variables|Default|GetDoor_OGLocation) "0, 0, 0" 1.0 1.0 0.0 0 0 0 0)
    (CallFunction|EnterOpenDoor (Variables|DoorOpen&CloseEvents|GetDungeonDoor_OGRotation) (Math|Rotator|MakeRotator (.roll _dungeondoor_ogrotation) (.pitch _dungeondoor_ogrotation) (Math|Float|ClampAngle (- (.yaw _dungeondoor_ogrotation) _opendoor_rotangle) 0.0 _opendoor_rotangle)) (Variables|DoorOpen&CloseEvents|GetRotator))
    (else
      (Audio|PlaySoundatLocation "/Game/ClassicMansion/Audio/Cues/SC_DoorClose.SC_DoorClose" (Variables|Default|GetDoor_OGLocation) "0, 0, 0" 1.0 1.0 0.0 0 0 0 0)
      (Variables|Door_Open&Close_Events|SetDoor_CurRotation (Transformation|GetWorldRotation (Variables|DoorOpen&CloseEvents|GetRotator)))
      (CallFunction|EnterCloseDoor (Variables|DoorOpen&CloseEvents|GetRotator) (Variables|Door_Open&Close_Events|GetDoor_CurRotation) (Math|Rotator|MakeRotator (.roll (Variables|Door_Open&Close_Events|GetDoor_CurRotation)) (.pitch (Variables|Door_Open&Close_Events|GetDoor_CurRotation)) (Math|Float|ClampAngle (+ (.yaw (Variables|Door_Open&Close_Events|GetDoor_CurRotation)) _opendoor_rotangle_2) 0.0 (* _opendoor_rotangle_2 -1.0)))))))

(fn ConstructionScript
  (|CallParentFunction))