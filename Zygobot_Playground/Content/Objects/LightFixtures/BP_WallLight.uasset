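; BP_WallLight is a wall light fixture that flickers while a spook event is active.
; Activate and Deactivate toggle a SpookOn flag, which Tick checks every frame to run either the flicker or the restore event.
; Flickering alternates the light's visibility and intensity between hidden and original states using short random delays.
; The exit event restores visibility and the intensity saved at BeginPlay after a similar delay.
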(event Custom|Enter_FlickerLight
  (bind _wallflickerlight (Variables|Default|GetWallFlickerLight))
  (bind _wallflickerlight_2 (Variables|Default|GetWallFlickerLight))
  (bind _wallflickerlight_3 (Variables|Default|GetWallFlickerLight))
  ;[0.151 0.1205 0] Flicker Lights
  (Rendering|SetVisibility _wallflickerlight_2 false false)
  (Rendering|Components|Light|SetIntensity _wallflickerlight_2 (Variables|Default|GetFlicker_Intensity))
  (Utilities|FlowControl|Delay (Math|Random|RandomFloatinRange 0.1 0.25))
  (Rendering|SetVisibility _wallflickerlight true false)
  (Rendering|Components|Light|SetIntensity _wallflickerlight (Variables|Default|GetOG_Intensity))
  (Utilities|FlowControl|Delay (Math|Random|RandomFloatinRange 0.1 0.25))
  (Rendering|SetVisibility _wallflickerlight_3 false false)
  (Rendering|Components|Light|SetIntensity _wallflickerlight_3 (Variables|Default|GetFlicker_Intensity)))

(event Custom|Exit_FlickerLight
  (bind _wallflickerlight (Variables|Default|GetWallFlickerLight))
  ;[0.1094 0.09271 0] End light flicker
  (Utilities|FlowControl|Delay (Math|Random|RandomFloatinRange 0.1 0.25))
  (Rendering|SetVisibility _wallflickerlight true false)
  (Rendering|Components|Light|SetIntensity _wallflickerlight (Variables|Default|GetOG_Intensity)))

(event EventBeginPlay
  ;[0 0.006612 0.09375] BEGIN PLAY events
  (Variables|Default|SetOG_Intensity (Variables|/Script/Engine.LightComponentBase|GetIntensity (Variables|Default|GetWallFlickerLight))))

(event EventTick
  (params (DeltaSeconds :type Float%20%28single-precision%29))
  (if (Variables|Default|GetbSpookOn?)
    (CallFunction|EnterFlickerLight)
    (else
      (CallFunction|ExitFlickerLight))))

(event EventActivate
  ;[0.1667 0.008673 0] Spook event Activate
  (Variables|Default|SetbSpookOn? true))

(event EventDeactivate
  ;[0.1615 0 0] Spook event Deactivate
  (Variables|Default|SetbSpookOn? false))

(fn ConstructionScript)