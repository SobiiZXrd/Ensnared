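; Roof light fixture whose twelve lights flicker together while a spook event is active.
; Activate and Deactivate toggle SpookOn, which Tick checks every frame to run the flicker or restore visibility and intensity.
; The flicker alternates hidden lights at FlickerIntensity with visible lights at the original intensity, using random short Delays.
; BeginPlay caches that original intensity from one light and applies it to all on restore.
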(event Custom|Enter_FlickerLight
  (bind _roofflickerlight (Variables|Default|GetRoofFlickerLight))
  ;[0.151 0.1205 0] Flicker Lights
  (Rendering|SetVisibility (Variables|Default|GetRoofFlickerLight1) false false)
  (Rendering|Components|Light|SetIntensity _roofflickerlight (Variables|Default|GetFlicker_Intensity))
  (Utilities|FlowControl|Delay (Math|Random|RandomFloatinRange 0.1 0.5))
  (Rendering|SetVisibility _roofflickerlight true false)
  (Rendering|Components|Light|SetIntensity _roofflickerlight (Variables|Default|GetOG_Intensity))
  (Utilities|FlowControl|Delay (Math|Random|RandomFloatinRange 0.1 0.5))
  (Rendering|SetVisibility _roofflickerlight false false)
  (Rendering|Components|Light|SetIntensity _roofflickerlight (Variables|Default|GetFlicker_Intensity)))

(event Custom|Exit_FlickerLight
  ;[0.1094 0.09271 0] End light flicker
  (Rendering|SetVisibility (Variables|Default|GetRoofFlickerLight1) true false)
  (Rendering|Components|Light|SetIntensity (Variables|Default|GetRoofFlickerLight) (Variables|Default|GetOG_Intensity)))

(event EventBeginPlay
  ;[0 0.006612 0.09375] BEGIN PLAY events
  (Variables|Default|SetOG_Intensity (Variables|/Script/Engine.LightComponentBase|GetIntensity (Variables|Default|GetRoofFlickerLight))))

(event EventTick
  (params (DeltaSeconds :type Float%20%28single-precision%29))
  ;[0 0.0625 0.005553] PER FRAME EVENTS: Spook Flicker
  (if (Variables|Default|GetbSpookOn?)
    (CallFunction|EnterFlickerLight)
    (else
      (CallFunction|ExitFlickerLight))))

(event EventActivate
  ;[0.1667 0.008673 0] Spook event Activate
  (Variables|Default|SetbSpookOn? true))

(event EventDeactivate
  ;[0.1615 0 0] Spook event Deactivate
  (Variables|Default|SetbSpookOn? false))

(fn ConstructionScript)