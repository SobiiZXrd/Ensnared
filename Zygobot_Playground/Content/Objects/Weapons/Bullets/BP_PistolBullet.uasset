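; BP_PistolBullet is a pistol projectile that deals damage and credits it to the player's controller and character.
; Collision overlaps apply standard damage only to actors tagged Enemy, without destroying the bullet.
; Blocking hits call destroy on the bullet, then apply point damage to whatever was struck, with no tag check.
; That point damage passes the impact point as the hit direction.
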(event OnComponentBeginOverlap(CollisionComponent)
  (params (OverlappedComponent :type Primitive%20Component%20Object%20Reference) (OtherActor :type Actor%20Object%20Reference) (OtherComp :type Primitive%20Component%20Object%20Reference) (OtherBodyIndex :type Integer) (bFromSweep :type Boolean) (SweepResult :type Hit%20Result%20Structure%20%28by%20ref%29))
  (bind (_playerchar_ref _playercontrol_ref) (CallFunction|GetPlayerCharacterP))
  ;[0.07292 0.07292 0.07292] Bullet damage and destroy self events
  (bind _output_get (Variables|BulletDamage|SetShotActor OtherActor))
  (if (Actor|ActorHasTag _output_get "Enemy")
    (Game|Damage|ApplyDamage (Variables|BulletDamage|GetShotActor) (Variables|BulletDamage|GetBase%20Damage) _playercontrol_ref _playerchar_ref)))

(event OnComponentHit(CollisionComponent)
  (params (HitComponent :type Primitive%20Component%20Object%20Reference) (OtherActor :type Actor%20Object%20Reference) (OtherComp :type Primitive%20Component%20Object%20Reference) (NormalImpulse :type Vector :default "0, 0, 0") (Hit :type Hit%20Result%20Structure%20%28by%20ref%29))
  (bind (_playerchar_ref _playercontrol_ref) (CallFunction|GetPlayerCharacterP))
  ;[0.07292 0.07292 0.07292] Bullet damage and destroy self events
  (Actor|DestroyActor)
  (Game|Damage|ApplyPointDamage OtherActor (Variables|BulletDamage|GetBase%20Damage) (.ImpactPoint (Collision|BreakHitResult Hit)) Hit _playercontrol_ref _playerchar_ref))

(event EventBeginPlay)

(fn ConstructionScript
  (|CallParentFunction))