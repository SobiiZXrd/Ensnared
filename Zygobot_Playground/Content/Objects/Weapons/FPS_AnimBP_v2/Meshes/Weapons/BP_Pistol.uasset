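; Pistol weapon Blueprint that the test character can equip and fire.
; FEquip runs only if the character's AnimBP HasPistol flag is unset, setting it and snapping the pistol to the right-hand object socket.
; FAction spawns a pistol-owned BP_PistolBullet at BulletSpawn, regardless of collision, and plays a gunshot sound there.
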(event EventBeginPlay)

(event EventFEquip
  (bind (_playerchar_ref _playercontrol_ref _animbp_ref) (CallFunction|GetAnimTestCharacter))
  (bind _right_hand (Variables|/Game/Character/Player/BP_AnimTestZ.BP_AnimTestZ_C|GetRight_Hand _playerchar_ref))
  (if (not (Variables|/Game/Character/AnimStarterPack/Mixamo/ABP_ZMix.ABP_ZMix_C|GetbHasPistol? _animbp_ref))
    (Variables|/Game/Character/AnimStarterPack/Mixamo/ABP_ZMix.ABP_ZMix_C|SetbHasPistol? _animbp_ref true)
    (Transformation|AttachComponentToComponent _right_hand (Class|SkinnedMeshComponent|GetSocketBoneName _right_hand "RightHand_ObjectSocket") "SnapToTarget" "SnapToTarget" "KeepWorld" true)))

(event EventFAction
  (bind _bulletspawn (Variables|Default|GetBulletSpawn))
  (bind _returnvalue (Transformation|GetWorldTransform _bulletspawn))
  (Game|SpawnActorfromClass "/Game/Objects/Weapons/Bullets/BP_PistolBullet.BP_PistolBullet_C" (Math|Transform|MakeTransform (.location _returnvalue) (.rotation _returnvalue) "1.000000,1.000000,1.000000") "AlwaysSpawn" self 0)
  (Audio|PlaySoundatLocation "/Game/Systems/Sound/WAV_Dump/427592__michorvath__9mm-pistol-shot.427592__michorvath__9mm-pistol-shot" (.location _returnvalue) (.rotation _returnvalue) 1.0 1.0 0.0 0 0 self 0))

(fn ConstructionScript)